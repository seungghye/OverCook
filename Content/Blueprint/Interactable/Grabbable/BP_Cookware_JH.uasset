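; BP_Cookware_JH is a grabbable cookware interactable that runs timed cooking with a progress bar widget.
; Cook stores whether cooking is allowed and starts it from zero progress when enabled and Items is not empty.
; While cooking, Tick shows the widget and advances Progress at a constant SlicingSpeed, updating WBP_ProgressBar_JH and debug-printing the value.
; At full progress it calls StopCooking and hides the widget.
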(event `self.ReceiveBeginPlay`
  (`SceneComponent.SetVisibility` (`self.Widget`) false false))

(event `self.ReceiveTick`
  (params (DeltaSeconds :type "Float (single-precision)"))
  (`parent.ReceiveTick` DeltaSeconds)
  (if (`self.IsCooking`)
    (`SceneComponent.SetVisibility` (`self.Widget`) true false)
    (`self.SetProgress` DeltaSeconds)
    (if (== (`self.Progress`) 1.0)
      (`/Game/Data/BPI_Interactable_JH.StopCooking`)
      (`SceneComponent.SetVisibility` (`self.Widget`) false false))))

(event `/Game/Data/BPI_Cookware.Cook`
  (params (Enable :type Boolean))
  (bind _output_get (set `self.IsCanCooking` Enable))
  (if (and _output_get (`KismetMathLibrary.Conv_IntToBool` (`KismetArrayLibrary.Array_Length` (`self.Items`))))
    (set `self.IsCooking` true)
    (set `self.Progress` 0.0)))

(fn `SetProgress`
  (params (DeltaSeconds :type "Float (double-precision)"))
  (bind _output_get (set `self.Progress` (`KismetMathLibrary.FInterpTo_Constant` (`self.Progress`) 1.0 DeltaSeconds (`self.SlicingSpeed`))))
  (bind _aswbp_progress_bar_jh (cast `/Game/Widget/Stage/WBP_ProgressBar_JH` (`WidgetComponent.GetUserWidgetObject` (`self.Widget`))))
  (`/Game/Widget/Stage/WBP_ProgressBar_JH.SetProgress` _aswbp_progress_bar_jh _output_get)
  (`KismetSystemLibrary.PrintString` (`KismetStringLibrary.Conv_DoubleToString` _output_get) true true (struct :`G` 0.66 :`B` 1.0 :`A` 1.0) DeltaSeconds))

(fn `UserConstructionScript`
  (`parent.UserConstructionScript`))