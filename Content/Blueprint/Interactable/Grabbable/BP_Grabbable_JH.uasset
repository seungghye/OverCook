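; Grabbable interactable actor that a player can pick up and release, built on a physics Box and a Mesh.
; GrabandDrop only handles grabbing: it checks the player's grabbed-object state, then disables physics and collision and passes itself to the player's Grab.
; Drop is a separate event that detaches the actor in world space and restores Box physics and collision on both components.
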(event `/Game/Data/BPI_Interactable_JH.GrabAndDrop`
  (params (Player :type "/Game/GameMode/Stage/BP_Character_JH Object Reference"))
  (if (`self.CanBeGrabbed` Player)
    (`self.Grab` Player)))

(event `Drop`
  (bind _box (`self.Box`))
  (`self.K2_DetachFromActor` "KeepWorld" "KeepWorld" "KeepWorld")
  (`PrimitiveComponent.SetSimulatePhysics` _box true)
  (`PrimitiveComponent.SetCollisionEnabled` _box "QueryAndPhysics")
  (`PrimitiveComponent.SetCollisionEnabled` (`self.Mesh`) "QueryAndPhysics"))

(event `Grab`
  (params (Player :type "/Game/GameMode/Stage/BP_Character_JH Object Reference"))
  (`self.RemovePhysics`)
  (`/Game/GameMode/Stage/BP_Character_JH.Grab` Player self))

(fn `CanBeGrabbed`
  (params (Player :type "/Game/GameMode/Stage/BP_Character_JH Object Reference"))
  (returns (CanBeGrabbed :type Boolean))
  (return (not (`/Game/GameMode/Stage/BP_Character_JH.Get Grabbed Object` Player))))

(fn `RemovePhysics`
  (bind _box (`self.Box`))
  (`PrimitiveComponent.SetSimulatePhysics` _box false)
  (`PrimitiveComponent.SetCollisionEnabled` _box "NoCollision")
  (`PrimitiveComponent.SetCollisionEnabled` (`self.Mesh`) "NoCollision"))

(fn `UserConstructionScript`)