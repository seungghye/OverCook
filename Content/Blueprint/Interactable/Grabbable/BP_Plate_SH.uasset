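; Grabbable plate that holds food items and reports its contents as ingredients.
; AddItem runs the parent logic, then changes the food's state if it reports being sliced.
; GetIngredients tallies Items into a map of ingredient structs keyed by food asset, incrementing the amount for repeats and keeping the first state recorded for each.
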(event `/Game/Data/BPI_Dish_JH.AddItem`
  (params (FoodItem :type "/Game/Blueprint/Interactable/Grabbable/BP_Food_JH Object Reference"))
  (`parent.AddItem` FoodItem)
  (bind _isslicenow (`/Game/Blueprint/Interactable/Grabbable/BP_Food_JH.IsSliceNow` FoodItem))
  (if _isslicenow
    (`/Game/Blueprint/Interactable/Grabbable/BP_Food_JH.SetState` FoodItem "NewEnumerator2")))

(fn `GetIngredients`
  (returns (Ingredients :type "Map of /Game/Data/FoodItem/DA_Food_Item_BP Object Reference to /Game/Data/ST_Ingredient Structure"))
  (locals (PlateIngredient :type "Map of /Game/Data/FoodItem/DA_Food_Item_BP Object Reference to /Game/Data/ST_Ingredient Structure") (FoodItems :type "/Game/Blueprint/Interactable/Grabbable/BP_Food_JH Object Reference"))
  (bind _fooditems (`local.FoodItems`))
  (for _array_element (`self.Items`)
    ;[1 1 1 1 15] 이거 두개  연결해주세요. Food_JH랑 Food_SH병합 이후
    (bind _output_get (set `local.FoodItems` _array_element))
    (bind (_value _returnvalue) (`BlueprintMapLibrary.Map_Find` (`local.PlateIngredient`) (`/Game/Blueprint/Interactable/Grabbable/BP_Food_JH.FoodItemAsset` _output_get)))
    (if _returnvalue
      (`BlueprintMapLibrary.Map_Add` (`local.PlateIngredient`) (`/Game/Blueprint/Interactable/Grabbable/BP_Food_JH.FoodItemAsset` (`local.FoodItems`)) (make `/Game/Data/ST_Ingredient` (break `/Game/Data/ST_Ingredient` _value) (+ (`.Amount_32_E56828F94FB039E0485A0A9893929FEF` (break `/Game/Data/ST_Ingredient` _value)) 1)))
      (else
        (`BlueprintMapLibrary.Map_Add` (`local.PlateIngredient`) (`/Game/Blueprint/Interactable/Grabbable/BP_Food_JH.FoodItemAsset` _fooditems) (make `/Game/Data/ST_Ingredient` (`/Game/Blueprint/Interactable/Grabbable/BP_Food_JH.State` _fooditems) 1)))))
  (return (`local.PlateIngredient`)))

(fn `UserConstructionScript`
  (`parent.UserConstructionScript`))