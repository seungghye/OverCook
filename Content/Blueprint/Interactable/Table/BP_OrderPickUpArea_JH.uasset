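; Order pick-up area interactable where players hand in plated food as a submitted order.
; GrabandDrop compares the held plate's ingredients against a test recipe list; on a match it destroys the plate and adds one to a plate box.
; The plate box is the assigned one or, if invalid, a random one gathered at BeginPlay.
; Only with authority does it report the matched food to the stage game mode, flagged as pick-up.
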(event `self.ReceiveBeginPlay`
  (`self.PlateBox`
    (:`then`)
    (:`else`
      (bind _outactors (`GameplayStatics.GetAllActorsOfClass` "/Game/Blueprint/Interactable/Table/BP_PlateBox_JH.BP_PlateBox_JH_C"))
      (set `self.AllPlateBoxes` _outactors))))

(event `/Game/Data/BPI_Interactable_JH.GrabAndDrop`
  (params (Player :type "/Game/GameMode/Stage/BP_Character_JH Object Reference"))
  (bind _asbp_plate_sh (cast `/Game/Blueprint/Interactable/Grabbable/BP_Plate_SH` (`.GrabbedObject` (`/Game/GameMode/Stage/BP_Character_JH.Get Grabbed Object` Player))))
  (if (not (`/Game/Blueprint/Interactable/Grabbable/BP_Kitchenware_JH.IsEmpty` _asbp_plate_sh))
    (for _array_element (`self.RecipeForTest`)
      (if (`/Game/Data/Recipe/DA_Recipe_BP.Compare` _array_element (`/Game/Blueprint/Interactable/Grabbable/BP_Plate_SH.GetIngredients` _asbp_plate_sh))
        (`self.K2_DestroyActor` _asbp_plate_sh)
        (set `/Game/GameMode/Stage/BP_Character_JH.GrabbedObject` null Player)
        (`/Game/Blueprint/Interactable/Table/BP_PlateBox_JH.AddPlate` (`self.GetCurPlateBox`))
        (`/Engine/EditorBlueprintResources/ActorMacros.Switch Has Authority`
          (:`Authority`
            (`self.ReqSubmitFood` _array_element)
            (break)))))))

(event `ReqSubmitFood`
  (params (SubmittedFood :type "/Game/Data/Recipe/DA_Recipe_BP Object Reference"))
  (bind _asbp_stage_game_mode_yj (cast `/Game/GameMode/Stage/BP_StageGameMode_YJ` (`GameplayStatics.GetGameMode`)))
  (`/Game/GameMode/Stage/BP_StageGameMode_YJ.SubmitFood` _asbp_stage_game_mode_yj SubmittedFood true))

(fn `GetCurPlateBox`
  (returns (PlateBox :type "/Game/Blueprint/Interactable/Table/BP_PlateBox_JH Object Reference"))
  (bind _platebox (`self.PlateBox`)
    (:`then`
      (return _platebox))
    (:`else`
      (return (`KismetArrayLibrary.Array_Random` (`self.AllPlateBoxes`))))))

(fn `UserConstructionScript`)