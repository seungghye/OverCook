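; Interactable food dispenser, built on a parent Blueprint, that hands a player a new food item from its FoodItemAsset.
; Grab/Drop spawns only when no valid PlaceObject is present and the player holds nothing; an occupied dispenser takes no action here.
; A Req/Res event pair calls SpawnFood, which spawns BP_Food_JH and immediately makes the player grab it.
; The construction script sets the top mesh's material from the food's icon.
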(event `Grab/Drop_1`
  (params (Player :type "/Game/GameMode/Stage/BP_Character_JH Object Reference"))
  (bind _placeobject (`self.PlaceObject`)
    (:`then`
      (if (`/Game/Blueprint/Interactable/Grabbable/BP_Grabbable_JH.CanBeGrabbed` _placeobject Player)
        _))
    (:`else`
      (if (not (`/Game/GameMode/Stage/BP_Character_JH.Get Grabbed Object` Player))
        (`self.ReqSpawnFood` Player)))))

(event `ReqSpawnFood`
  (params (Player :type "/Game/GameMode/Stage/BP_Character_JH Object Reference"))
  (`self.ResSpawnFood` Player))

(event `ResSpawnFood`
  (params (Player :type "/Game/GameMode/Stage/BP_Character_JH Object Reference"))
  (`self.SpawnFood` Player))

(fn `SpawnFood`
  (params (Player :type "/Game/GameMode/Stage/BP_Character_JH Object Reference"))
  (bind _returnvalue (`|SpawnActorFromClass` "/Game/Blueprint/Interactable/Grabbable/BP_Food_JH.BP_Food_JH_C" (`self.GetTransform`) "Undefined" "MultiplyWithRoot" null true (`self.FoodItemAsset`) null))
  (`/Game/Data/BPI_Interactable_JH.GrabAndDrop` _returnvalue Player))

(fn `UserConstructionScript`
  (`parent.UserConstructionScript`)
  (`KismetMaterialLibrary.CreateDynamicMaterialInstance` "/Game/Asset/kitchen_Tools/Material/M_DarwerTomato.M_DarwerTomato")
  (`PrimitiveComponent.SetMaterial` (`self.SM_TOP`) 0 (`/Game/Data/FoodItem/DA_Food_Item_BP.Icon` (`self.FoodItemAsset`))))