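; Lobby stage marker that shows one stage's information and carries out travel to that stage.
; A box trigger shows or hides the info widget as a BP_LobbyTruckPawn enters or leaves.
; BeginPlay and the StageInfo RepNotify fill the widget with image, name, score and stars, and show a clear statue for positive scores.
; Travel requests store the stage in the GameInstance, disable player 0's pawn input and run a servertravel console command.
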(event `self.ReceiveBeginPlay`
  (`self.InitializeWidget`))

(event `self.BoxCollision.OnComponentBeginOverlap`
  (params (OverlappedComponent :type "PrimitiveComponent Object Reference") (OtherActor :type "Actor Object Reference") (OtherComp :type "PrimitiveComponent Object Reference") (OtherBodyIndex :type Integer) (bFromSweep :type Boolean) (SweepResult :type "HitResult Structure (by ref)"))
  (if (== (`GameplayStatics.GetObjectClass` OtherActor) "/Game/Blueprint/BP_LobbyTruckPawn.BP_LobbyTruckPawn_C")
    (`SceneComponent.SetVisibility` (`self.Widget`) true false)))

(event `self.BoxCollision.OnComponentEndOverlap`
  (params (OverlappedComponent :type "PrimitiveComponent Object Reference") (OtherActor :type "Actor Object Reference") (OtherComp :type "PrimitiveComponent Object Reference") (OtherBodyIndex :type Integer))
  (if (== (`GameplayStatics.GetObjectClass` OtherActor) "/Game/Blueprint/BP_LobbyTruckPawn.BP_LobbyTruckPawn_C")
    (`SceneComponent.SetVisibility` (`self.Widget`) false false)))

(event `ReqTravelStage`
  (bind _returnvalue (`GameplayStatics.GetPlayerController` 0))
  (bind _asbp_over_cook_game_instance_yj (cast `/Game/GameMode/BP_OverCookGameInstance_YJ` (`GameplayStatics.GetGameInstance`)))
  (set `/Game/GameMode/BP_OverCookGameInstance_YJ.SelectedStage` (`self.StageInfo`) _asbp_over_cook_game_instance_yj)
  (`self.DisableInput` (`Controller.K2_GetPawn` _returnvalue) _returnvalue)
  ;[1 1 1] 이동할 '맵 이름' 주의
  (`KismetSystemLibrary.PrintString` "Stage : Run ExecuteConsoleCommand !" true true (struct :`R` 1.0 :`B` 0.884576 :`A` 1.0) 60.0)
  (`KismetSystemLibrary.ExecuteConsoleCommand` (`KismetStringLibrary.Concat_StrStr` "servertravel " (`.StageName_14_5A7A2F1347E1E665CB5C40A1F6A6CD38` (break `/Game/Data/LobbyData/ST_StageInfo` (`self.StageInfo`)))) null))

(fn `CheckClear`
  (bind _clearstatue (`self.ClearStatue`))
  (if (> (`.LastScore_18_42F39F314AFE4BDCED90C88C65511ED1` (break `/Game/Data/LobbyData/ST_StageInfo` (`self.StageInfo`))) 0)
    (`SceneComponent.SetVisibility` _clearstatue true false)
    (else
      (`SceneComponent.SetVisibility` _clearstatue false false))))

(fn `InitializeWidget`
  (locals (InfoWidget :type "/Game/Widget/Lobby/WBP_StageInformation_YJ Object Reference"))
  (bind (_stageimage _stagename _recipemenu _lastscore) (break `/Game/Data/LobbyData/ST_StageInfo` (`self.StageInfo`)))
  (bind _aswbp_stage_information_yj (cast `/Game/Widget/Lobby/WBP_StageInformation_YJ` (`WidgetComponent.GetUserWidgetObject` (`self.Widget`))))
  (set `local.InfoWidget` _aswbp_stage_information_yj)
  (`|ExecutionSequence`
    (:`then_0`
      (bind _astexture_2d (cast `Texture2D` _stageimage))
      (`/Game/Widget/Lobby/WBP_StageInformation_YJ.SetStageImage` (`local.InfoWidget`) _astexture_2d))
    (:`then_1`
      (`/Game/Widget/Lobby/WBP_StageInformation_YJ.SetStageName` (`local.InfoWidget`) (`KismetTextLibrary.Conv_StringToText` _stagename)))
    (:`then_2`
      (`/Game/Widget/Lobby/WBP_StageInformation_YJ.SetScoreText` (`local.InfoWidget`) _lastscore)
      (`self.CheckClear`))
    (:`then_3`
      (`/Game/Widget/Lobby/WBP_StageInformation_YJ.SetScoreStar` (`local.InfoWidget`) _lastscore))))

(fn `OnRep_StageInfo`
  (`self.InitializeWidget`))

(fn `TravelStage`
  (bind _returnvalue (`GameplayStatics.GetPlayerController` 0))
  (bind _asbp_over_cook_game_instance_yj (cast `/Game/GameMode/BP_OverCookGameInstance_YJ` (`GameplayStatics.GetGameInstance`)))
  (set `/Game/GameMode/BP_OverCookGameInstance_YJ.SelectedStage` (`self.StageInfo`) _asbp_over_cook_game_instance_yj)
  (`self.DisableInput` (`Controller.K2_GetPawn` _returnvalue) _returnvalue)
  ;[1 1 1] 이동할 '맵 이름' 주의
  (`KismetSystemLibrary.PrintString` "Stage : Run ExecuteConsoleCommand !" true true (struct :`R` 1.0 :`B` 0.884576 :`A` 1.0) 60.0)
  (`KismetSystemLibrary.ExecuteConsoleCommand` (`KismetStringLibrary.Concat_StrStr` "servertravel " (`.StageName_14_5A7A2F1347E1E665CB5C40A1F6A6CD38` (break `/Game/Data/LobbyData/ST_StageInfo` (`self.StageInfo`)))) null))

(fn `UserConstructionScript`)