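; BP_StageController2_JH is a controller that places its BP_Character_JH pawn, and those of its peer controllers, at PlayerStarts on BeginPlay.
; BeginPlay passes through a Req/Res event pair into SetPlayerStart0.
; That function gathers every controller of this class and teleports each one's pawn to the location and rotation of the PlayerStart with the same array index.
; A failed character cast stops the function.
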(event `self.ReceiveBeginPlay`
  (`self.ReqSetPlayerStart`)
  (`parent.ReceiveBeginPlay`))

(event `ReqSetPlayerStart`
  (`self.ResSetPlayerStart`))

(event `ResSetPlayerStart`
  (`self.SetPlayerStart_0`))

(fn `SetPlayerStart_0`
  (bind _outactors (`GameplayStatics.GetAllActorsOfClass` "BP_StageController2_JH_C"))
  (for (_array_element _array_index) _outactors
    (bind _outactors_2 (`GameplayStatics.GetAllActorsOfClass` "/Script/Engine.PlayerStart"))
    (for (_array_element_2 _array_index_2) _outactors_2
      (if (== _array_index_2 _array_index)
        (bind _asbp_character_jh (cast `/Game/Common/GameMode/Stage/BP_Character_JH` (`self.K2_GetPawn` _array_element)))
        (bind (_returnvalue_location _returnvalue_rotation) (`KismetMathLibrary.BreakTransform` (`self.GetTransform` _array_element_2)))
        (`self.K2_SetActorLocationAndRotation` _asbp_character_jh _returnvalue_location _returnvalue_rotation false true)))))

(fn `UserConstructionScript`
  (`parent.UserConstructionScript`))