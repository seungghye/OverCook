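; BP_StageGM2_JH is a stage game mode that registers players into the user list held by BP_StageGameState2_JH.
; AddUserList fills the first slot lacking a valid controller with the passed controller, an empty name and a connected flag.
; It then calls the game state's CallEventDispatcherUserList to broadcast the change.
; BeginPlay and the construction script only call their parent versions.
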(event `self.ReceiveBeginPlay`
  (`parent.ReceiveBeginPlay`))

(fn `AddUserList`
  (params (NewParam :type "PlayerController Object Reference"))
  (locals (GameState :type "/Game/JH/GameMode/BP_StageGameState2_JH Object Reference"))
  (bind _asbp_stage_game_state_2_jh (cast `/Game/JH/GameMode/BP_StageGameState2_JH` (`GameplayStatics.GetGameState`)))
  (set `local.GameState` _asbp_stage_game_state_2_jh)
  (bind _userlist (`/Game/JH/GameMode/BP_StageGameState2_JH.UserList` _asbp_stage_game_state_2_jh))
  (for (_array_element _array_index) _userlist
    (`/Engine/EditorBlueprintResources/StandardMacros.IsValid` (`.UserController_4_11A49D354753C45B956708A595C981A3` (break `/Game/Common/Data/LobbyData/ST_UserList` _array_element))
      (:`Is Not Valid`
        (`KismetArrayLibrary.Array_Set` _userlist _array_index (make `/Game/Common/Data/LobbyData/ST_UserList` "" NewParam true))
        (`/Game/JH/GameMode/BP_StageGameState2_JH.EventDispatcher_UserList` (`local.GameState`))
        (return)))))

(fn `UserConstructionScript`
  (`parent.UserConstructionScript`))