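; Game mode that assigns a player start to each player on login and prints the player's name.
; On PostLogin, SetPlayerStart loops over all PlayerStart actors, skipping those recorded in the UsedPlayerStarts map.
; It teleports the PlayerController, not its pawn, to each unused start and records it.
; The loop has no break, so one login claims every free start.
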(event `self.K2_PostLogin`
  (params (NewPlayer :type "PlayerController Object Reference"))
  (`self.SetPlayerStart` NewPlayer)
  (`KismetSystemLibrary.PrintString` (`AdvancedSessionsLibrary.GetPlayerName` NewPlayer)))

(fn `SetPlayerStart`
  (params (PlayerController :type "PlayerController Object Reference"))
  (bind _outactors (`GameplayStatics.GetAllActorsOfClass` "/Script/Engine.PlayerStart"))
  (for _array_element _outactors
    (if (not (`.ReturnValue` (`BlueprintMapLibrary.Map_Find` (`self.UsedPlayerStarts`) _array_element)))
      (bind (_returnvalue_location _returnvalue_rotation) (`KismetMathLibrary.BreakTransform` (`self.GetTransform` _array_element)))
      (`self.K2_SetActorLocationAndRotation` PlayerController _returnvalue_location _returnvalue_rotation false true)
      (`BlueprintMapLibrary.Map_Add` (`self.UsedPlayerStarts`) _array_element))))

(fn `UserConstructionScript`)