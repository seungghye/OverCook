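; Grabbable interactable actor that a player can pick up and drop.
; Grab proceeds only if the player's grabbed-object check is false, disabling physics and collision on the sphere component before passing itself to the player's Grab.
; Drop detaches the actor at its world transform and restores sphere physics simulation and query-and-physics collision.
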(event `/Game/JH/Blueprints/Data/BPI_Interactable_JH.Grab`
  (params (Player :type "/Game/JH/Blueprints/Data/BP_Character_JH Object Reference"))
  (bind _spherecollision (`self.SphereCollision`))
  (if (not (`/Game/JH/Blueprints/Data/BP_Character_JH.Get Grabbed Object` Player))
    (`PrimitiveComponent.SetSimulatePhysics` _spherecollision false)
    (`PrimitiveComponent.SetCollisionEnabled` _spherecollision "NoCollision")
    (`/Game/JH/Blueprints/Data/BP_Character_JH.Grab` Player self)))

(event `Drop`
  (bind _spherecollision (`self.SphereCollision`))
  (`self.K2_DetachFromActor` "KeepWorld" "KeepWorld" "KeepWorld")
  (`PrimitiveComponent.SetSimulatePhysics` _spherecollision true)
  (`PrimitiveComponent.SetCollisionEnabled` _spherecollision "QueryAndPhysics"))

(fn `UserConstructionScript`)