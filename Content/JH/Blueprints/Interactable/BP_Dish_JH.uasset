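; BP_Dish_JH is a dish that collects food items up to a maximum count.
; AddItem stores the FoodItem in the Items array, attaches it to the FoodPlace component keeping its world transform, then moves its root with MoveComponentTo.
; HasPlace reports whether Items is below MaxItemCount, a limit that AddItem itself does not check.
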(event `/Game/JH/Blueprints/Data/BPI_Dish_JH.AddItem`
  (params (FoodItem :type "/Game/JH/Blueprints/Interactable/BP_Food_JH Object Reference"))
  (`KismetArrayLibrary.Array_Add` (`self.Items`) FoodItem)
  (`self.K2_AttachToComponent` FoodItem (`self.FoodPlace`) "None" "KeepWorld" "KeepWorld" "KeepWorld" true)
  (`KismetSystemLibrary.MoveComponentTo` (`Actor.RootComponent` FoodItem)))

(fn `HasPlace`
  (returns (HasPlace :type Boolean))
  (return (< (`KismetArrayLibrary.Array_Length` (`self.Items`)) (`self.MaxItemCount`))))

(fn `UserConstructionScript`
  (`parent.UserConstructionScript`))