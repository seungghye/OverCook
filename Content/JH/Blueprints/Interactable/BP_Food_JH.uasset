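; BP_Food_JH is an interactable food actor that tracks a slicing state of Raw, Slicing or Sliced.
; SetState stores the state and swaps the Sphere's material to match, a temporary visual that a note says will become an anim montage.
; IsCanSlice returns true only when the IsSlice flag is set and the food is not yet Sliced.
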(event `SetState`
  (params (State :type "/Game/JH/Blueprints/Data/EN_Foodstate Enum" :default "NewEnumerator0"))
  (bind _output_get (set `self.State` State))
  (`PrimitiveComponent.SetMaterial` (`self.Sphere`) 0 (select `/Game/JH/Blueprints/Data/EN_Foodstate` _output_get :`NewEnumerator1` "/Game/JH/Materials/KeyDiskMaterial.KeyDiskMaterial" :`NewEnumerator2` "/Game/JH/Materials/MAT_LevelColorationLitLightmapUV.MAT_LevelColorationLitLightmapUV" :!type "Material Object Reference")))

(fn `IsCanSlice`
  (returns (IsSlice :type Boolean))
  (return (and (`self.IsSlice`) (select `/Game/JH/Blueprints/Data/EN_Foodstate` (`self.State`) :`NewEnumerator0` true :`NewEnumerator1` true))))

(fn `UserConstructionScript`
  (`parent.UserConstructionScript`))