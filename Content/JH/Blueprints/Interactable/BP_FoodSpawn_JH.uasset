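; BP_FoodSpawn_JH is an interactable food dispenser that also keeps its parent's grab and drop behavior.
; With no PlaceObject and an empty-handed player, it spawns a BP_Food_JH at its own transform and immediately grabs it for that player.
; If the player already holds something, or a valid PlaceObject can be grabbed, it defers to the parent Grab/Drop logic.
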(event `/Game/JH/Blueprints/Data/BPI_Interactable_JH.Grab/Drop`
  (params (Player :type "/Game/JH/Blueprints/Data/BP_Character_JH Object Reference"))
  (bind _placeobject (`self.PlaceObject`)
    (:`then`
      (if (`/Game/JH/Blueprints/Interactable/BP_Grabbable_JH.CanBeGrabbed` _placeobject Player)
        (`parent.Grab/Drop` Player :!label _label)))
    (:`else`
      (if (`/Game/JH/Blueprints/Data/BP_Character_JH.Get Grabbed Object` Player)
        (goto _label)
        (else
          (bind _returnvalue (`|SpawnActorFromClass` "/Game/JH/Blueprints/Interactable/BP_Food_JH.BP_Food_JH_C" (`self.GetTransform`) "Undefined" "MultiplyWithRoot" null true null))
          (`/Game/JH/Blueprints/Data/BPI_Interactable_JH.Grab/Drop` _returnvalue Player))))))

(fn `UserConstructionScript`
  (`parent.UserConstructionScript`))