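; BP_CuttingBoard_JH is an interactable cutting board where a player slices a placed BP_Food_JH.
; Cooking checks that the food can be sliced, changes its state and flags the player as cooking.
; Tick fills Progress at SlicingSpeed, debug-printing it, then stops cooking and advances the food's state at completion.
; Grab is allowed only at zero or full Progress, then resets it.
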(event `self.ReceiveBeginPlay`
  (`parent.ReceiveBeginPlay`))

(event `self.ReceiveActorBeginOverlap`
  (params (OtherActor :type "Actor Object Reference"))
  (`parent.ReceiveActorBeginOverlap` OtherActor))

(event `self.ReceiveTick`
  (params (DeltaSeconds :type "Float (single-precision)"))
  (`parent.ReceiveTick` DeltaSeconds)
  (if (`self.IsInteracting`)
    (bind _output_get (set `self.Progress` (`KismetMathLibrary.FInterpTo_Constant` (`self.Progress`) 1.0 DeltaSeconds (`self.SlicingSpeed`))))
    (`KismetSystemLibrary.PrintString` (`KismetStringLibrary.Conv_DoubleToString` _output_get) true true (struct :`G` 0.66 :`B` 1.0 :`A` 1.0) DeltaSeconds)
    (if (== (`self.Progress`) 1.0)
      (`/Game/JH/Blueprints/Data/BPI_Interactable_JH.StopCooking`)
      (bind _asbp_food_jh (cast `/Game/JH/Blueprints/Interactable/BP_Food_JH` (`self.PlaceObject`)))
      (`/Game/JH/Blueprints/Interactable/BP_Food_JH.SetState` _asbp_food_jh "NewEnumerator2"))))

(event `/Game/JH/Blueprints/Data/BPI_Interactable_JH.Grab`
  (params (Player :type "/Game/JH/Blueprints/Data/BP_Character_JH Object Reference"))
  (if (`self.CanGrabObject`)
    (`parent.Grab` Player)
    (set `self.Progress` 0.0)))

(event `/Game/JH/Blueprints/Data/BPI_Interactable_JH.Cooking`
  (params (Player :type "/Game/JH/Blueprints/Data/BP_Character_JH Object Reference"))
  (bind _asbp_food_jh (cast `/Game/JH/Blueprints/Interactable/BP_Food_JH` (`self.PlaceObject`)))
  (if (`/Game/JH/Blueprints/Interactable/BP_Food_JH.IsCanSlice` _asbp_food_jh)
    (`/Game/JH/Blueprints/Interactable/BP_Food_JH.SetState` _asbp_food_jh "NewEnumerator1")
    (`/Game/JH/Blueprints/Data/BP_Character_JH.SetIsCooking` Player true self)
    (set `self.InteractingPlayer` Player)
    (set `self.IsInteracting` true)))

(event `/Game/JH/Blueprints/Data/BPI_Interactable_JH.StopCooking`
  (set `self.IsInteracting` false)
  (`/Game/JH/Blueprints/Data/BP_Character_JH.SetIsCooking` (`self.InteractingPlayer`) false null))

(fn `CanGrabObject`
  (returns (ReturnValue :type Boolean))
  (return (or (== (`self.Progress`) 0.0) (== (`self.Progress`) 1.0))))

(fn `UserConstructionScript`
  (`parent.UserConstructionScript`))