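; BP_OrderPickUpArea_JH is an interactable pick-up area that takes non-empty plates from players and returns them to a plate box.
; On Grab/Drop, a held BP_Plate_JH with contents is destroyed and AddPlate is called on a plate box.
; The box is the assigned PlateBox, or a random one from all BP_PlateBox_JH actors gathered at BeginPlay when none is set.
; No order checking or scoring happens here.
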(event `self.ReceiveBeginPlay`
  (`self.PlateBox`
    (:`then`)
    (:`else`
      (bind _outactors (`GameplayStatics.GetAllActorsOfClass` "/Game/JH/Blueprints/Interactable/Table/BP_PlateBox_JH.BP_PlateBox_JH_C"))
      (set `self.AllPlateBoxes` _outactors))))

(event `/Game/JH/Blueprints/Data/BPI_Interactable_JH.Grab/Drop`
  (params (Player :type "/Game/JH/Blueprints/Data/BP_Character_JH Object Reference"))
  (bind _asbp_plate_jh (cast `/Game/JH/Blueprints/Interactable/Grabbable/BP_Plate_JH` (`.GrabbedObject` (`/Game/JH/Blueprints/Data/BP_Character_JH.Get Grabbed Object` Player))))
  (if (not (`/Game/JH/Blueprints/Interactable/Grabbable/BP_Dish_JH.IsEmpty` _asbp_plate_jh))
    (`self.K2_DestroyActor` _asbp_plate_jh)
    (`/Game/JH/Blueprints/Interactable/Table/BP_PlateBox_JH.AddPlate` (`self.GetCurPlateBox`))))

(fn `GetCurPlateBox`
  (returns (PlateBox :type "/Game/JH/Blueprints/Interactable/Table/BP_PlateBox_JH Object Reference"))
  (bind _platebox (`self.PlateBox`)
    (:`then`
      (return _platebox))
    (:`else`
      (return (`KismetArrayLibrary.Array_Random` (`self.AllPlateBoxes`))))))

(fn `UserConstructionScript`)