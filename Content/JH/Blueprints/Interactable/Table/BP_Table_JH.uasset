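; BP_Table_JH is an interactable table that holds one object, which players can put down or pick up.
; Grab/Drop checks the player's hands: empty hands take the table's object, while a held object goes onto an empty table.
; If both are occupied, the table's object handles the grab itself when CanBeGrabbed allows.
; Placing attaches the object to the ObjectPlace component, moves it with MoveComponentTo and clears the player's GrabbedObject.
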(event `/Game/JH/Blueprints/Data/BPI_Interactable_JH.Grab/Drop`
  (params (Player :type "/Game/JH/Blueprints/Data/BP_Character_JH Object Reference"))
  (bind (_isgetgrabbedobject _grabbedobject) (`/Game/JH/Blueprints/Data/BP_Character_JH.Get Grabbed Object` Player))
  (if _isgetgrabbedobject
    (bind _placeobject (`self.PlaceObject`)
      (:`then`
        (if (`/Game/JH/Blueprints/Interactable/Grabbable/BP_Grabbable_JH.CanBeGrabbed` _placeobject Player)
          (`/Game/JH/Blueprints/Interactable/Grabbable/BP_Grabbable_JH.Grab` (`self.PlaceObject`) Player)
          (set `self.PlaceObject` null)))
      (:`else`
        (`self.Place` _grabbedobject Player)))
    (else
      (`self.Grab` Player))))

(event `Place`
  (params (ObjectToPlace :type "/Game/JH/Blueprints/Interactable/Grabbable/BP_Grabbable_JH Object Reference") (Player :type "/Game/JH/Blueprints/Data/BP_Character_JH Object Reference"))
  (bind _output_get (set `self.PlaceObject` ObjectToPlace))
  (`self.K2_AttachToComponent` _output_get (`self.ObjectPlace`) "None" "KeepWorld" "KeepWorld" "KeepWorld" true)
  (`KismetSystemLibrary.MoveComponentTo` (`Actor.RootComponent` (`self.PlaceObject`)))
  (set `/Game/JH/Blueprints/Data/BP_Character_JH.GrabbedObject` null Player))

(event `Grab`
  (params (Player :type "/Game/JH/Blueprints/Data/BP_Character_JH Object Reference"))
  (`/Engine/EditorBlueprintResources/StandardMacros.IsValid` (`self.PlaceObject`)
    (:`Is Valid`
      (`/Game/JH/Blueprints/Data/BP_Character_JH.Grab` Player (`self.PlaceObject`))
      (set `self.PlaceObject` null))))

(fn `UserConstructionScript`)