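; BP_PlateBox_JH is an interactable plate dispenser that holds a stack of plates for players to take.
; On BeginPlay it spawns a default number of BP_Plate_JH actors, disables their physics and attaches them at ObjectPlace, offsetting each by plate height.
; On Grab/Drop it hands the top plate to the player if that plate can be grabbed, then removes it from the array.
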(event `self.ReceiveBeginPlay`
  (`self.InitPlates`))

(event `/Game/JH/Blueprints/Data/BPI_Interactable_JH.Grab/Drop`
  (params (Player :type "/Game/JH/Blueprints/Data/BP_Character_JH Object Reference"))
  (bind _plates (`self.Plates`))
  (if (`KismetArrayLibrary.Array_IsNotEmpty` (`self.Plates`))
    (if (`/Game/JH/Blueprints/Interactable/Grabbable/BP_Grabbable_JH.CanBeGrabbed` (`|GetArrayItem` _plates (`KismetArrayLibrary.Array_LastIndex` _plates)) Player)
      (`self.Grab` Player))))

(event `self.Grab`
  (params (Player :type "/Game/JH/Blueprints/Data/BP_Character_JH Object Reference"))
  (bind _plates (`self.Plates`))
  (bind _output (`|GetArrayItem` _plates (`KismetArrayLibrary.Array_LastIndex` _plates)))
  (`/Game/JH/Blueprints/Interactable/Grabbable/BP_Grabbable_JH.Grab` _output Player)
  (`KismetArrayLibrary.Array_RemoveItem` (`self.Plates`) _output))

(fn `AddPlate`
  (bind (_returnvalue_x _returnvalue_y _returnvalue_z) (`KismetMathLibrary.BreakVector` (`SceneComponent.K2_GetComponentLocation` (`self.ObjectPlace`))))
  (bind _returnvalue (`|SpawnActorFromClass` "/Game/JH/Blueprints/Interactable/Grabbable/BP_Plate_JH.BP_Plate_JH_C" (`KismetMathLibrary.MakeTransform` (`KismetMathLibrary.MakeVector` _returnvalue_x _returnvalue_y (+ _returnvalue_z (* (`KismetArrayLibrary.Array_Length` (`self.Plates`)) (`self.PlateHeight`))))) "Undefined" "MultiplyWithRoot" null null))
  (`/Game/JH/Blueprints/Interactable/Grabbable/BP_Grabbable_JH.RemovePhysics` _returnvalue)
  (`self.K2_AttachToComponent` _returnvalue (`self.ObjectPlace`) "None" "KeepWorld" "KeepWorld" "KeepWorld" true)
  (`KismetArrayLibrary.Array_Add` (`self.Plates`) _returnvalue))

(fn `InitPlates`
  (for _ (range 1 (+ (`self.DefaultPlatesAmount`) 1))
    (`self.AddPlate`)))

(fn `UserConstructionScript`
  (`parent.UserConstructionScript`))