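; Grabbable dish that collects food items from the player, up to a maximum item count.
; It can be grabbed by an empty-handed player, or by one holding grabbable food while the dish has space.
; Grab first adds any held food, attaching it to FoodPlace in world space and moving it with MoveComponentTo, then runs the parent grab.
; An OnDestroy handler destroys the contained food along with the dish.
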(event `self.ReceiveBeginPlay`
  (`parent.ReceiveBeginPlay`)
  (add `self.OnDestroyed` (`|CreateDelegate` :!event `OnDestroy`)))

(event `/Game/JH/Blueprints/Data/BPI_Dish_JH.AddItem`
  (params (FoodItem :type "/Game/JH/Blueprints/Interactable/Grabbable/BP_Food_JH Object Reference"))
  (`KismetArrayLibrary.Array_Add` (`self.Items`) FoodItem)
  (`self.K2_AttachToComponent` FoodItem (`self.FoodPlace`) "None" "KeepWorld" "KeepWorld" "KeepWorld" true)
  (`KismetSystemLibrary.MoveComponentTo` (`Actor.RootComponent` FoodItem)))

(event `self.Grab`
  (params (Player :type "/Game/JH/Blueprints/Data/BP_Character_JH Object Reference"))
  (`self.AddFoodFromCharacter` Player)
  (`parent.Grab` Player))

(fn `AddFoodFromCharacter`
  (params (Target :type "/Game/JH/Blueprints/Data/BP_Character_JH Object Reference"))
  (bind (_isgetgrabbedobject _grabbedobject) (`/Game/JH/Blueprints/Data/BP_Character_JH.Get Grabbed Object` Target))
  (if _isgetgrabbedobject
    (bind _asbp_food_jh (cast `/Game/JH/Blueprints/Interactable/Grabbable/BP_Food_JH` _grabbedobject))
    (`self.AddItem` _asbp_food_jh)))

(fn `CanBeGrabbed`
  (params (Player :type "/Game/JH/Blueprints/Data/BP_Character_JH Object Reference"))
  (returns (CanBeGrabbed :type Boolean))
  (bind (_isgetgrabbedobject _grabbedobject) (`/Game/JH/Blueprints/Data/BP_Character_JH.Get Grabbed Object` Player))
  (if (not _isgetgrabbedobject)
    (return true)
    (else
      (bind _asbp_food_jh (cast `/Game/JH/Blueprints/Interactable/Grabbable/BP_Food_JH` _grabbedobject)
        (:`then`
          (if (`/Game/JH/Blueprints/Interactable/Grabbable/BP_Food_JH.IsCanGrab` _asbp_food_jh)
            (return (`self.HasPlace`))))
        (:`CastFailed`
          (return false))))))

(fn `HasPlace`
  (returns (HasPlace :type Boolean))
  (return (< (`KismetArrayLibrary.Array_Length` (`self.Items`)) (`self.MaxItemCount`))))

(fn `IsEmpty`
  (returns (ReturnValue :type Boolean))
  (return (`KismetArrayLibrary.Array_IsEmpty` (`self.Items`))))

(fn `OnDestroy`
  (params (DestroyedActor :type "Actor Object Reference"))
  (for _array_element (`self.Items`)
    (`self.K2_DestroyActor` _array_element)))

(fn `UserConstructionScript`
  (`parent.UserConstructionScript`))