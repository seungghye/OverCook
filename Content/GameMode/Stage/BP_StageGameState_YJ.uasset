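; Stage game state for a recipe-order game, tracking remaining time, score, stage state and the ordered recipe list.
; RepNotify handlers for time, score and stage state fire event dispatchers, as do recipe adds and removals, which exist as both events and functions.
; The order list caps at five, and AddScore also counts successful or failed orders by the score's sign.
; An author note flags that add broadcasts may precede HUD binding.
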(event `ResAddOrderedRecipe`
  (params (OrderedRecipe :type "/Game/Data/Recipe/DA_Recipe_BP Object Reference"))
  (bind _orderedrecipelist (`self.OrderedRecipeList`))
  (if (< (`KismetArrayLibrary.Array_Length` _orderedrecipelist) 5)
    (`KismetArrayLibrary.Array_Add` _orderedrecipelist OrderedRecipe)
    ;[1 1 1] 시작후 HUD바인드 되기 전에 호출될까봐 걱정된다. 예외처리 필요할듯
    (`self.EventDispatcher_AddOrderedRecipe` OrderedRecipe)))

(event `ResSubtractOrderRecipe`
  (params (RecipeIndex :type Integer))
  (`KismetArrayLibrary.Array_Remove` (`self.OrderedRecipeList`) RecipeIndex)
  (`self.EventDispatcher_SubtractOrderedRecipe` RecipeIndex))

(fn `AddOrderedRecipe`
  (params (OrdededRecipe :type "/Game/Data/Recipe/DA_Recipe_BP Object Reference (by ref)"))
  (bind _orderedrecipelist (`self.OrderedRecipeList`))
  (if (< (`KismetArrayLibrary.Array_Length` _orderedrecipelist) 5)
    (`KismetArrayLibrary.Array_Add` _orderedrecipelist OrdededRecipe)
    ;[1 1 1] 시작후 HUD바인드 되기 전에 호출될까봐 걱정된다. 예외처리 필요할듯
    (`self.EventDispatcher_AddOrderedRecipe` OrdededRecipe)))

(fn `AddScore`
  (params (InScore :type Integer))
  (set `self.Score` (+ (`self.Score`) InScore))
  (`self.IsSuccessOrder` (> InScore 0)))

(fn `DecreaseLeftTime`
  (set `self.LeftTime` (- (`self.LeftTime`) 1)))

(fn `IsSuccessOrder`
  (params (IsSuccess :type Boolean))
  (if IsSuccess
    (set `self.CntSuccessOrder` (+ (`self.CntSuccessOrder`) 1))
    (else
      (set `self.CntFailedOrder` (+ (`self.CntFailedOrder`) 1)))))

(fn `OnRep_LeftTime`
  (`self.EventDispatcher_LeftTime` (`self.LeftTime`)))

(fn `OnRep_Score`
  (`self.EventDispatcher_Score` (`self.Score`)))

(fn `OnRep_StageState`
  (`self.EventDispatcher_StageState` (`self.StageState`)))

(fn `SetStageState`
  (params (StageState :type "/Game/Data/EN_StageState Enum" :default "NewEnumerator0"))
  (set `self.StageState` StageState))

(fn `SubtractOrderedRecipe`
  (params (RecipeIndex :type Integer))
  (`KismetArrayLibrary.Array_Remove` (`self.OrderedRecipeList`) RecipeIndex)
  (`self.EventDispatcher_SubtractOrderedRecipe` RecipeIndex))

(fn `UserConstructionScript`)