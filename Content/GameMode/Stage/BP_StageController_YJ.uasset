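; Player controller for stages that gates pawn input by stage state and places characters at player starts.
; On BeginPlay it binds to the stage game state, retrying on a timer until available, and enables pawn input only during Play.
; It also adds the input mapping context and teleports each stage controller's character to the PlayerStart with the matching array index.
; Cheat nodes for submitting food and adding orders are left unconnected.
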(event Custom|ReqSetPlayerStart
  (CallFunction|ResSetPlayerStart))

(event Custom|ResSetPlayerStart
  (CallFunction|SetPlayerStart))

(event EventBeginPlay
  (Utilities|FlowControl|Sequence
    (:then_0
      (CallFunction|BindGameState))
    (:then_1
      (Input|AddMappingContext (PlayerController|LocalPlayerSubsystems|GetEnhancedInputLocalPlayerSubsystem (Game|GetPlayerController 0)) "/Game/Input/Stage/IMC_Default_JH.IMC_Default_JH" 0 "(bIgnoreAllPressedKeysUntilRelease=True,bForceImmediately=False,bNotifyUserSettings=False)"))
    (:then_2
      (CallFunction|ReqSetPlayerStart))))

(event Input|KeyboardEvents|DebugKeyF
  (params (Key :type Key%20Structure) (ActionValue :type Input%20Action%20Value%20Structure))
  ;[1 1 1] Cheat Key
)

(event Input|KeyboardEvents|DebugKeyG
  (params (Key :type Key%20Structure) (ActionValue :type Input%20Action%20Value%20Structure))
  ;[1 1 1] Cheat Key
)

(fn ConstructionScript)

(fn BindGameState
  (bind _asbp_stage_game_state_yj (Utilities|Casting|CastToBP_StageGameState_YJ (Game|GetGameState))
    (:then
      (EventDispatchers|BindEventtoEventDispatcherStageState _asbp_stage_game_state_yj (EventDispatchers|CreateEvent :!event SetControllerInput))
      (CallFunction|SetControllerInput (Variables|/Game/GameMode/Stage/BP_StageGameState_YJ.BP_StageGameState_YJ_C|GetStageState _asbp_stage_game_state_yj)))
    (:CastFailed
      (Utilities|Time|SetTimerbyFunctionName 0 "BindGameState" 0.1))))

(fn SetControllerInput
  (params (StageState :type EN_StageState%20Enum :default "NewEnumerator0"))
  (bind _self self)
  (bind _self_2 self)
  (bind _self_3 self)
  (bind _returnvalue (Pawn|GetControlledPawn _self_2))
  (switch Utilities|FlowControl|Switch|SwitchonEN_StageState StageState
    (:NewEnumerator0
      (Utilities|IsValid _returnvalue
        (:Is%20Valid
          (Input|DisableInput _returnvalue _self_2))))
    (:NewEnumerator1
      (Input|EnableInput (Pawn|GetControlledPawn _self) _self))
    (:NewEnumerator2
      (Input|DisableInput (Pawn|GetControlledPawn _self_3) _self_3))))

(fn SetPlayerStart
  (bind _outactors (Actor|GetAllActorsOfClass "BP_StageController_YJ_C"))
  (for (_array_element _array_index) _outactors
    (bind _outactors_2 (Actor|GetAllActorsOfClass "/Script/Engine.PlayerStart"))
    (for (_array_element_2 _array_index_2) _outactors_2
      (if (== _array_index_2 _array_index)
        (bind _asbp_character_jh (Utilities|Casting|CastToBP_Character_JH (Pawn|GetControlledPawn _array_element)))
        (Transformation|SetActorLocationAndRotation _asbp_character_jh (.location (Transformation|GetActorTransform _array_element_2)) (.rotation (Transformation|GetActorTransform _array_element_2)) false true)))))