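; Game mode for an Overcooked-style cooking stage, running the match from ready countdown through play to scoreboard and server travel back to the lobby.
; It seeds the game state from the selected stage in the game instance, then timers tick down time and add random recipe orders.
; Submitted food is matched to orders by class to award score or a penalty.
; At time-out it disables player input and saves the score to the game instance.
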(event `self.ReceiveBeginPlay`
  (`self.IntializeGameState`)
  (`/Game/GameMode/Stage/BP_StageGameState_YJ.SetStageState` (`self.StageGameState`) "NewEnumerator0")
  (`KismetSystemLibrary.Delay` 3.0)
  (`self.StartStage`))

(fn `AddOrderedRecipe`
  (`/Game/GameMode/Stage/BP_StageGameState_YJ.ResAddOrderedRecipe` (`self.StageGameState`) (`KismetArrayLibrary.Array_Random` (`self.RecipeMenu`))))

(fn `AddScore`
  (params (InScore :type Integer))
  (`/Game/GameMode/Stage/BP_StageGameState_YJ.AddScore` (`self.StageGameState`) InScore))

(fn `BackToLobby`
  (`KismetSystemLibrary.PrintString` "Stage : Run ExecuteConsoleCommand !" true true (struct :`R` 1.0 :`B` 0.884576 :`A` 1.0) 60.0)
  (bind _asbp_over_cook_game_instance_yj (cast `/Game/GameMode/BP_OverCookGameInstance_YJ` (`GameplayStatics.GetGameInstance`)))
  ;[1 1 1] 맵이름 조심
  (`KismetSystemLibrary.ExecuteConsoleCommand` (`KismetStringLibrary.Concat_StrStr` "servertravel " (`/Game/GameMode/BP_OverCookGameInstance_YJ.LobbyStage` _asbp_over_cook_game_instance_yj)) null))

(fn `DoStageTimer`
  (bind _stagegamestate (`self.StageGameState`))
  (`/Game/GameMode/Stage/BP_StageGameState_YJ.DecreaseLeftTime` _stagegamestate)
  (if (<= (`/Game/GameMode/Stage/BP_StageGameState_YJ.LeftTime` _stagegamestate) 0)
    (`self.EndStage`)))

(fn `EndStage`
  (`|ExecutionSequence`
    (:`then_0`
      (`/Game/GameMode/Stage/BP_StageGameState_YJ.SetStageState` (`self.StageGameState`) "NewEnumerator2")
      (`KismetSystemLibrary.K2_PauseTimer` null "DoStageTimer")
      (`KismetSystemLibrary.K2_PauseTimer` null "AddOrderedRecipe"))
    (:`then_1`
      ;[1 1 1] 모든 유저 disable input
      (bind _outactors (`GameplayStatics.GetAllActorsOfClass` "/Script/Engine.PlayerController"))
      (for _array_element _outactors
        (`self.DisableInput` _array_element)))
    (:`then_2`
      (bind _asbp_over_cook_game_instance_yj (cast `/Game/GameMode/BP_OverCookGameInstance_YJ` (`GameplayStatics.GetGameInstance`)))
      (`/Game/GameMode/BP_OverCookGameInstance_YJ.UpdateStages` _asbp_over_cook_game_instance_yj (`/Game/GameMode/Stage/BP_StageGameState_YJ.Score` (`self.StageGameState`)))
      (`KismetSystemLibrary.K2_SetTimer` null "BackToLobby" 10.0))))

(fn `IntializeGameState`
  (locals (GameInstance :type "/Game/GameMode/BP_OverCookGameInstance_YJ Object Reference"))
  (bind (_stageimage _stagename _recipemenu _lastscore _timelimit) (break `/Game/Data/LobbyData/ST_StageInfo` (`/Game/GameMode/BP_OverCookGameInstance_YJ.SelectedStage` (`local.GameInstance`))))
  (bind _asbp_stage_game_state_yj (cast `/Game/GameMode/Stage/BP_StageGameState_YJ` (`GameplayStatics.GetGameState`))
    (:`then`
      (set `self.StageGameState` _asbp_stage_game_state_yj)
      (bind _asbp_over_cook_game_instance_yj (cast `/Game/GameMode/BP_OverCookGameInstance_YJ` (`GameplayStatics.GetGameInstance`)))
      (set `local.GameInstance` _asbp_over_cook_game_instance_yj)
      (`|ExecutionSequence`
        (:`then_0`
          (set `/Game/GameMode/Stage/BP_StageGameState_YJ.LeftTime` _timelimit (`self.StageGameState`)))
        (:`then_1`
          (set `/Game/GameMode/Stage/BP_StageGameState_YJ.StageName` _stagename (`self.StageGameState`)))
        (:`then_2`
          ;[1 1 1] GM의 변수 초기화
          (set `self.RecipeMenu` _recipemenu))
        (:`then_3`
          ;[1 1 1] OnRep위해 일단유지
          (set `/Game/GameMode/Stage/BP_StageGameState_YJ.Score` 0 (`self.StageGameState`)))))
    (:`CastFailed`
      (`KismetSystemLibrary.PrintString` "GM: GameState cast failed" true true (struct :`R` 1.0 :`G` 0.263207 :`A` 1.0) 60.0))))

(fn `SetStageState`
  (params (StageState :type "/Game/Data/EN_StageState Enum" :default "NewEnumerator0"))
  (bind _stagegamestate (`self.StageGameState`))
  (`/Game/GameMode/Stage/BP_StageGameState_YJ.SetStageState` _stagegamestate StageState)
  ;[1 1 1] 서버 OnRep 직접호출
  (`/Game/GameMode/Stage/BP_StageGameState_YJ.EventDispatcher_StageState` _stagegamestate StageState))

(fn `StartStage`
  (`self.SetStageState` "NewEnumerator1")
  (`KismetSystemLibrary.K2_SetTimer` null "DoStageTimer" 1.0 true)
  (`KismetSystemLibrary.K2_SetTimer` null "AddOrderedRecipe" (`self.OrderInterval`) true false (* (`self.OrderInterval`) -0.8)))

(fn `SubmitFood`
  (params (SubmittedFood :type "/Game/Data/Recipe/DA_Recipe_BP Object Reference") (IsSubmitByPickUp :type Boolean))
  ;[1 1 1] 여기는 무조건 허용. BP_PickUpArea에서 등록된 레시피인지 GameState에서 Req를 통해 검사하고 GameMode의 SubmitFood호출하자.
  ;[1 1 1] ScoreBoard동안에 음식타이머로 점수바뀌는것 제한
  (switch `/Game/Data/EN_StageState` (`/Game/GameMode/Stage/BP_StageGameState_YJ.StageState` (`self.StageGameState`))
    (:`NewEnumerator1`
      (if IsSubmitByPickUp
        (bind _issuccess (`self.SubtractOrderedRecipe` SubmittedFood))
        (if _issuccess
          (`self.AddScore` (`/Game/Data/Recipe/DA_Recipe_BP.Score` SubmittedFood))
          (else
            (`self.AddScore` -100 :!label _label)))
        (else
          (`self.SubtractOrderedRecipe` SubmittedFood)
          (goto _label))))))

(fn `SubtractOrderedRecipe`
  (params (SubmittedFood :type "/Game/Data/Recipe/DA_Recipe_BP Object Reference"))
  (returns (IsSuccess :type Boolean))
  (for (_array_element _array_index) (`/Game/GameMode/Stage/BP_StageGameState_YJ.OrderedRecipeList` (`self.StageGameState`))
    (if (== (`GameplayStatics.GetObjectClass` _array_element) (`GameplayStatics.GetObjectClass` SubmittedFood))
      (`/Game/GameMode/Stage/BP_StageGameState_YJ.ResSubtractOrderRecipe` (`self.StageGameState`) _array_index)
      (return true)))
  (return false))

(fn `UserConstructionScript`)