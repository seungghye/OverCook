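; Stage HUD that creates the stage widget and shows the countdown, score, recipe order sheets, state messages and end-of-stage results.
; It binds to BP_StageGameState_YJ event dispatchers, pushing changes into the widget and seeding time, score and state immediately.
; Timers clear the start text and reveal the result board after time out.
; If the GameState cast fails, the retry timer names BindWidgets, which is absent here, instead of BindGameState.
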(event `self.ReceiveBeginPlay`
  (bind _returnvalue (`|CreateWidget` "/Game/Widget/Stage/WBP_StageHudWidget_YJ.WBP_StageHudWidget_YJ_C"))
  (bind _output_get (set `self.HudWidget` _returnvalue))
  (`UserWidget.AddToViewport` _output_get 0)
  (`self.BindGameState`))

(fn `AddOrderedRecipe`
  (params (OrderedRecipe :type "/Game/Data/Recipe/DA_Recipe_BP Object Reference"))
  (`/Game/Widget/Stage/WBP_StageHudWidget_YJ.AddOrderSheet` (`self.HudWidget`) OrderedRecipe))

(fn `BindGameState`
  (locals (StageGameState :type "/Game/GameMode/Stage/BP_StageGameState_YJ Object Reference"))
  (bind _stagegamestate (`local.StageGameState`))
  (bind _stagegamestate_2 (`local.StageGameState`))
  (bind _stagegamestate_3 (`local.StageGameState`))
  (bind _asbp_stage_game_state_yj (cast `/Game/GameMode/Stage/BP_StageGameState_YJ` (`GameplayStatics.GetGameState`))
    (:`then`
      (set `local.StageGameState` _asbp_stage_game_state_yj)
      (`|ExecutionSequence`
        (:`then_0`
          (add `/Game/GameMode/Stage/BP_StageGameState_YJ.EventDispatcher_LeftTime` _stagegamestate_3 (`|CreateDelegate` :!event `UpdateLeftTime`))
          (`self.UpdateLeftTime` (`/Game/GameMode/Stage/BP_StageGameState_YJ.LeftTime` _stagegamestate_3)))
        (:`then_1`
          (add `/Game/GameMode/Stage/BP_StageGameState_YJ.EventDispatcher_Score` _stagegamestate_2 (`|CreateDelegate` :!event `UpdateScore`))
          (`self.UpdateScore` (`/Game/GameMode/Stage/BP_StageGameState_YJ.Score` _stagegamestate_2)))
        (:`then_2`
          (add `/Game/GameMode/Stage/BP_StageGameState_YJ.EventDispatcher_AddOrderedRecipe` (`local.StageGameState`) (`|CreateDelegate` :!event `AddOrderedRecipe`)))
        (:`then_3`
          (add `/Game/GameMode/Stage/BP_StageGameState_YJ.EventDispatcher_SubtractOrderedRecipe` (`local.StageGameState`) (`|CreateDelegate` :!event `SubtractOrderedRecipe`)))
        (:`then_4`
          (add `/Game/GameMode/Stage/BP_StageGameState_YJ.EventDispatcher_StageState` _stagegamestate (`|CreateDelegate` :!event `Event Stage State`))
          (`self.Event Stage State` (`/Game/GameMode/Stage/BP_StageGameState_YJ.StageState` _stagegamestate)))))
    (:`CastFailed`
      (`KismetSystemLibrary.K2_SetTimer` null "BindWidgets" 0.01))))

(fn `ClearStateText`
  (set `/Game/Widget/Stage/WBP_StageHudWidget_YJ.StateText` "" (`self.HudWidget`)))

(fn `Event Stage State`
  (params (StageState :type "/Game/Data/EN_StageState Enum" :default "NewEnumerator0"))
  (bind _hudwidget (`self.HudWidget`))
  (switch `/Game/Data/EN_StageState` StageState
    (:`NewEnumerator0`
      (set `/Game/Widget/Stage/WBP_StageHudWidget_YJ.StateText` "Ready..." _hudwidget))
    (:`NewEnumerator1`
      (set `/Game/Widget/Stage/WBP_StageHudWidget_YJ.StateText` "Start!" _hudwidget)
      (`KismetSystemLibrary.K2_SetTimer` null "ClearStateText" 2.0))
    (:`NewEnumerator2`
      (set `/Game/Widget/Stage/WBP_StageHudWidget_YJ.StateText` "Time Out!" _hudwidget)
      (`KismetSystemLibrary.K2_SetTimer` null "EventTimeOut" 2.0))))

(fn `EventTimeOut`
  (locals (StageGameState :type "/Game/GameMode/Stage/BP_StageGameState_YJ Object Reference"))
  (bind _hudwidget (`self.HudWidget`))
  (bind _stagegamestate (`local.StageGameState`))
  (bind _asbp_stage_game_state_yj (cast `/Game/GameMode/Stage/BP_StageGameState_YJ` (`GameplayStatics.GetGameState`)))
  (set `local.StageGameState` _asbp_stage_game_state_yj)
  (set `/Game/Widget/Stage/WBP_StageHudWidget_YJ.StageName` (`/Game/GameMode/Stage/BP_StageGameState_YJ.StageName` _stagegamestate) _hudwidget)
  (`/Game/Widget/Stage/WBP_StageHudWidget_YJ.SetCntSuccessOrder` _hudwidget (`/Game/GameMode/Stage/BP_StageGameState_YJ.CntSuccessOrder` _stagegamestate))
  (`/Game/Widget/Stage/WBP_StageHudWidget_YJ.SetCntFailedOrder` _hudwidget (`/Game/GameMode/Stage/BP_StageGameState_YJ.CntFailedOrder` _stagegamestate))
  (`Widget.SetVisibility` (`/Game/Widget/Stage/WBP_StageHudWidget_YJ.Border_ResultBoard` _hudwidget) "Visible"))

(fn `SubtractOrderedRecipe`
  (params (RecipeIndex :type Integer))
  (`/Game/Widget/Stage/WBP_StageHudWidget_YJ.SubtractOrderSheet` (`self.HudWidget`) RecipeIndex))

(fn `UpdateLeftTime`
  (params (LeftTime :type Integer))
  (bind _returnvalue (mod LeftTime 60))
  (bind _hudwidget (`self.HudWidget`))
  (bind _returnvalue_2 (`KismetStringLibrary.Conv_IntToString` (/ LeftTime 60)))
  (bind _returnvalue_3 (`KismetStringLibrary.Conv_IntToString` _returnvalue))
  (if (> _returnvalue 9)
    (set `/Game/Widget/Stage/WBP_StageHudWidget_YJ.LeftTime` (`KismetStringLibrary.Concat_StrStr` _returnvalue_2 " : " _returnvalue_3) _hudwidget)
    (else
      (set `/Game/Widget/Stage/WBP_StageHudWidget_YJ.LeftTime` (`KismetStringLibrary.Concat_StrStr` _returnvalue_2 " : " (`KismetStringLibrary.Concat_StrStr` "0" _returnvalue_3)) _hudwidget))))

(fn `UpdateScore`
  (params (Score :type Integer))
  (set `/Game/Widget/Stage/WBP_StageHudWidget_YJ.Score` Score (`self.HudWidget`)))

(fn `UserConstructionScript`)