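; BP_LobbyPawn_YJ is a lobby pawn that rides along with the lobby truck pawn.
; On BeginPlay it finds the first BP_LobbyTruckPawn, copies its camera rotation and spring arm length and socket offset, then snaps itself onto the truck.
; If no truck exists yet, it retries on a short timer until one appears.
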(event `self.ReceiveBeginPlay`
  ;[1 1 1] 카메라 시점 문제시, Springarm 콜리젼 체크할것
  (`self.AttachToTruck`))

(fn `AttachToTruck`
  (locals (LobbyTruck :type "/Game/Blueprint/BP_LobbyTruckPawn Object Reference"))
  (bind _springarm (`self.SpringArm`))
  (bind _springarm_2 (`/Game/Blueprint/BP_LobbyTruckPawn.SpringArm` (`local.LobbyTruck`)))
  (bind _outactors (`GameplayStatics.GetAllActorsOfClass` "/Game/Blueprint/BP_LobbyTruckPawn.BP_LobbyTruckPawn_C"))
  (bind _output (`|GetArrayItem` _outactors))
  (`/Engine/EditorBlueprintResources/StandardMacros.IsValid` _output
    (:`Is Valid`
      (set `local.LobbyTruck` _output)
      (`|ExecutionSequence`
        (:`then_0`
          (`SceneComponent.K2_SetRelativeRotation` (`self.Camera`) (`SceneComponent.RelativeRotation` (`/Game/Blueprint/BP_LobbyTruckPawn.Camera` (`local.LobbyTruck`))) false false))
        (:`then_1`
          (set `SpringArmComponent.TargetArmLength` (`SpringArmComponent.TargetArmLength` _springarm_2) _springarm)
          (set `SpringArmComponent.SocketOffset` (`SpringArmComponent.SocketOffset` _springarm_2) _springarm))
        (:`then_2`
          (`self.K2_AttachToActor` (`local.LobbyTruck`) "None" "SnapToTarget" "SnapToTarget" "KeepRelative"))))
    (:`Is Not Valid`
      (`KismetSystemLibrary.K2_SetTimer` null "AttachToTruck" 0.01))))

(fn `UserConstructionScript`)