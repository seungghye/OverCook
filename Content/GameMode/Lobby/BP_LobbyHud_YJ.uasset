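; Lobby HUD that creates the lobby widget and handles its chat and user image display.
; It binds to the chat box's commit and the game state's user list dispatcher, and rebroadcasts Enter-committed text with the GameInstance user name through its own ChatCommitted dispatcher.
; AddChat forwards messages to the widget.
; On start it broadcasts an entry message and refreshes user images, retrying by timer until the widget is valid.
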(event `self.ReceiveBeginPlay`
  (bind _returnvalue (`|CreateWidget` "/Game/Widget/Lobby/WBP_LobbyHudWidget_YJ.WBP_LobbyHudWidget_YJ_C"))
  (bind _output_get (set `self.HudWidget` _returnvalue))
  (`UserWidget.AddToViewport` _output_get 0)
  (`self.BindWidgets`)
  (`self.InitializeWidget`))

(fn `AddChat`
  (params (UserName :type String) (Chat :type Text))
  (`/Game/Widget/Lobby/WBP_LobbyHudWidget_YJ.AddChat` (`self.HudWidget`) UserName Chat))

(fn `BindWidgets`
  (`|ExecutionSequence`
    (:`then_0`
      (add `EditableText.OnTextCommitted` (`/Game/Widget/Lobby/WBP_LobbyHudWidget_YJ.EditableText_ChatBox` (`self.HudWidget`)) (`|CreateDelegate` :!event `EventChatCommitted`)))
    (:`then_1`
      (bind _asbp_lobby_game_state_yj (cast `/Game/GameMode/Lobby/BP_LobbyGameState_YJ` (`GameplayStatics.GetGameState`))
        (:`then`
          (add `/Game/GameMode/Lobby/BP_LobbyGameState_YJ.EventDispatcher_UserList` _asbp_lobby_game_state_yj (`|CreateDelegate` :!event `UpdateUserImage`)))
        (:`CastFailed`
          (`KismetSystemLibrary.PrintString` "HUD : BindWidgets-GameState cast failed" true true (struct :`R` 1.0 :`B` 0.00868 :`A` 1.0) 60.0))))))

(fn `EventChatCommitted`
  (params (Text :type "Text (by ref)") (CommitMethod :type "ETextCommit Enum" :default "Default"))
  (switch `ETextCommit` CommitMethod
    (:`OnEnter`
      (bind _asbp_over_cook_game_instance_yj (cast `/Game/GameMode/BP_OverCookGameInstance_YJ` (`GameplayStatics.GetGameInstance`))
        (:`then`
          (`self.EventDispatcher_ChatCommitted` (`/Game/GameMode/BP_OverCookGameInstance_YJ.UserName` _asbp_over_cook_game_instance_yj) Text)
          (return))
        (:`CastFailed`
          (`KismetSystemLibrary.PrintString` "LobbyHud : GameInstance CastFailed" true true (struct :`G` 0.66 :`B` 1.0 :`A` 1.0) 60.0))))))

(fn `InitializeWidget`
  (`|ExecutionSequence`
    (:`then_0`
      ;[1 1 1] 첫 입장 시, 입장 메시지 위해 수동 Committ
      (bind _asbp_over_cook_game_instance_yj (cast `/Game/GameMode/BP_OverCookGameInstance_YJ` (`GameplayStatics.GetGameInstance`)))
      (`self.EventDispatcher_ChatCommitted` (`/Game/GameMode/BP_OverCookGameInstance_YJ.UserName` _asbp_over_cook_game_instance_yj) "[ Enter Lobby ]"))
    (:`then_1`
      (`self.UpdateUserImage`))))

(fn `UpdateUserImage`
  (bind _hudwidget (`self.HudWidget`)
    (:`then`
      (`/Game/Widget/Lobby/WBP_LobbyHudWidget_YJ.UpdateUserImage` _hudwidget))
    (:`else`
      (`KismetSystemLibrary.K2_SetTimer` null "UpdateUserImage" 0.01))))

(fn `UserConstructionScript`)