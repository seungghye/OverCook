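; Game instance for an Overcooked-style game that holds the stage list and the currently selected stage.
; UpdateStages finds the entries in the Stages array whose name matches the selected stage.
; It writes the new score into LastScore by reference only when it beats the stored value, so that field acts as a per-stage high score.
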(fn `UpdateStages`
  (params (Score :type Integer))
  (locals (CurrentStage :type "/Game/Data/LobbyData/ST_StageInfo Structure"))
  (for (_array_element _array_index) (`self.Stages`)
    (if (`KismetStringLibrary.EqualEqual_StrStr` (`.StageName_14_5A7A2F1347E1E665CB5C40A1F6A6CD38` (break `/Game/Data/LobbyData/ST_StageInfo` _array_element)) (`.StageName_14_5A7A2F1347E1E665CB5C40A1F6A6CD38` (break `/Game/Data/LobbyData/ST_StageInfo` (`self.SelectedStage`))))
      (bind _output (`|GetArrayItem` (`self.Stages`) _array_index))
      (if (< (`.LastScore_18_42F39F314AFE4BDCED90C88C65511ED1` (break `/Game/Data/LobbyData/ST_StageInfo` _output)) Score)
        (setmembers `/Game/Data/LobbyData/ST_StageInfo` :`StructRef` _output :`LastScore` Score)))))