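; Entry menu panel actor that moves the player's view to the create or join panel.
; On BeginPlay it casts its widget component's user widget to WBP_EntryMenuWidget_YJ and binds to that widget's Create and Join dispatchers.
; ClickCreate and ClickJoin use SetViewTargetWithBlend on player controller 0, so menu navigation is a timed camera blend between panel actors.
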(event `self.ReceiveBeginPlay`
  (`self.BindWidget`))

(fn `BindWidget`
  (locals (EntryMenuWidget :type "/Game/Common/Widget/Entry/WBP_EntryMenuWidget_YJ Object Reference"))
  (bind _aswbp_entry_menu_widget_yj (cast `/Game/Common/Widget/Entry/WBP_EntryMenuWidget_YJ` (`WidgetComponent.GetUserWidgetObject` (`self.Widget`))))
  (set `local.EntryMenuWidget` _aswbp_entry_menu_widget_yj)
  (`|ExecutionSequence`
    (:`then_0`
      (add `/Game/Common/Widget/Entry/WBP_EntryMenuWidget_YJ.EventDispatcher_Create` (`local.EntryMenuWidget`) (`|CreateDelegate` :!event `ClickCreate`)))
    (:`then_1`
      (add `/Game/Common/Widget/Entry/WBP_EntryMenuWidget_YJ.EventDispatcher_Join` (`local.EntryMenuWidget`) (`|CreateDelegate` :!event `ClickJoin`)))))

(fn `ClickCreate`
  (`PlayerController.SetViewTargetWithBlend` (`GameplayStatics.GetPlayerController` 0) (`self.CreatePanel`) (`self.BlendTime`) "VTBlend_Linear" 0.0 false))

(fn `ClickJoin`
  (`PlayerController.SetViewTargetWithBlend` (`GameplayStatics.GetPlayerController` 0) (`self.JoinPanel`) (`self.BlendTime`) "VTBlend_Linear" 0.0 false))

(fn `UserConstructionScript`
  (`parent.UserConstructionScript`))