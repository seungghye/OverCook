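; Cabbage drawer actor, apparently a kitchen ingredient dispenser, that reacts to actors overlapping it.
; Overlap start and end toggle CanInteract, tilt the Top component open and back, and print debug messages.
; The Z key only prints a debug string; the CanInteract check and BP_Ingredient spawn are unconnected, and IfInputCtrl is empty, so dispensing is unfinished.
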(event `self.ReceiveActorBeginOverlap`
  (params (OtherActor :type "Actor Object Reference"))
  (set `self.canInteract` true)
  (`KismetSystemLibrary.PrintString` "Overlap" true true (struct :`G` 0.66 :`B` 1.0 :`A` 1.0) 60.0)
  (`SceneComponent.K2_AddLocalRotation` (`self.Top`) (struct :`Pitch` 30.0) false false))

(event `self.ReceiveActorEndOverlap`
  (params (OtherActor :type "Actor Object Reference"))
  (set `self.canInteract` false)
  (`SceneComponent.K2_AddLocalRotation` (`self.Top`) (struct :`Pitch` -30.0) false false)
  (`KismetSystemLibrary.PrintString` "EndOverlap" true true (struct :`G` 0.66 :`B` 1.0 :`A` 1.0) 60.0))

(event `Key|Z`
  (params (Key :type "Key Structure"))
  (:`Pressed`
    (`KismetSystemLibrary.PrintString` "Hello" true true (struct :`G` 0.66 :`B` 1.0 :`A` 1.0) 60.0)))

(fn `IfInputCtrl`)

(fn `UserConstructionScript`)