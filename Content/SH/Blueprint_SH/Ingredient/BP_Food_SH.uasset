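; Grabbable food ingredient actor that moves through Raw, Sliced and OnPlate states.
; Its FoodItemAsset supplies a mesh per state, swapped by SetState as a temporary stand-in for planned montages.
; Slicing is allowed when IsSlice is set and it is not plated.
; It is grabbable by empty hands or a held dish with room, though Grab always removes physics and only attaches to empty-handed players.
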(event `self.ReceiveBeginPlay`
  (`parent.ReceiveBeginPlay`)
  (`StaticMeshComponent.SetStaticMesh` (`self.Mesh`) (`/Game/SH/DT_SH/DA_Food_Item_BP.DefultMesh` (`self.FoodItemAsset`))))

(event `SetState`
  (params (State :type "/Game/JH/Blueprints/Data/EN_Foodstate_JH Enum" :default "NewEnumerator0"))
  (bind _fooditemasset (`self.FoodItemAsset`))
  (bind _output_get (set `self.State` State))
  (`StaticMeshComponent.SetStaticMesh` (`self.Mesh`) (select `/Game/JH/Blueprints/Data/EN_Foodstate_JH` _output_get :`NewEnumerator0` (`/Game/SH/DT_SH/DA_Food_Item_BP.DefultMesh` _fooditemasset) :`NewEnumerator1` (`/Game/SH/DT_SH/DA_Food_Item_BP.SlicedMesh` _fooditemasset) :`NewEnumerator2` (`/Game/SH/DT_SH/DA_Food_Item_BP.OnPlateMesh` _fooditemasset))))

(event `self.Grab`
  (params (Player :type "/Game/JH/Blueprints/Data/BP_Character_JH Object Reference"))
  (`self.RemovePhysics`)
  (if (not (`/Game/JH/Blueprints/Data/BP_Character_JH.Get Grabbed Object` Player))
    (`/Game/JH/Blueprints/Data/BP_Character_JH.Grab` Player self)))

(fn `CanBeGrabbed`
  (params (Player :type "/Game/JH/Blueprints/Data/BP_Character_JH Object Reference"))
  (returns (CanBeGrabbed :type Boolean))
  (bind (_isgetgrabbedobject _grabbedobject) (`/Game/JH/Blueprints/Data/BP_Character_JH.Get Grabbed Object` Player))
  (if (not _isgetgrabbedobject)
    (return true)
    (else
      (bind _asbp_dish_jh (cast `/Game/JH/Blueprints/Interactable/Grabbable/BP_Dish_JH` _grabbedobject)
        (:`then`
          (return (`/Game/JH/Blueprints/Interactable/Grabbable/BP_Dish_JH.HasPlace` _asbp_dish_jh)))
        (:`CastFailed`
          (return false))))))

(fn `IsCanSlice`
  (returns (IsSlice :type Boolean))
  (return (and (`self.IsSlice`) (select `/Game/JH/Blueprints/Data/EN_Foodstate_JH` (`self.State`) :`NewEnumerator0` true :`NewEnumerator1` true))))

(fn `UserConstructionScript`
  (`parent.UserConstructionScript`))