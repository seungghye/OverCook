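; BP_Plate_SH is a plate that holds food items and reports its contents as ingredients.
; AddItem extends the parent behavior by setting each added food item's state.
; GetIngredients tallies Items into a map keyed by food asset, storing a state and amount and keeping the first recorded state for duplicates.
; Developer notes mark some GetIngredients wiring as pending the merge of Food_JH and Food_SH.
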(event `/Game/JH/Blueprints/Data/BPI_Dish_JH.AddItem`
  (params (FoodItem :type "/Game/JH/Blueprints/Interactable/Grabbable/BP_Food_JH Object Reference"))
  (`parent.AddItem` FoodItem)
  (`/Game/JH/Blueprints/Interactable/Grabbable/BP_Food_JH.SetState` FoodItem "NewEnumerator3"))

(fn `GetIngredients`
  (returns (Ingredients :type "Map of /Game/SH/DT_SH/DA_Food_Item_BP Object Reference to /Game/SH/DT_SH/ST_Ingredient Structure"))
  (locals (PlateIngredient :type "Map of /Game/SH/DT_SH/DA_Food_Item_BP Object Reference to /Game/SH/DT_SH/ST_Ingredient Structure") (FoodItems :type "/Game/JH/Blueprints/Interactable/Grabbable/BP_Food_JH Object Reference"))
  (bind (_value _returnvalue) (`BlueprintMapLibrary.Map_Find` (`local.PlateIngredient`) (`/Game/SH/Blueprint_SH/Ingredient/BP_Food_SH.FoodItemAsset`)))
  (for _array_element (`self.Items`)
    ;[1 1 1 1 15] 이거 두개  연결해주세요. Food_JH랑 Food_SH병합 이후
    (set `local.FoodItems` _array_element)
    (if _returnvalue
      (`BlueprintMapLibrary.Map_Add` (`local.PlateIngredient`) (`/Game/SH/Blueprint_SH/Ingredient/BP_Food_SH.FoodItemAsset`) (make `/Game/SH/DT_SH/ST_Ingredient` (break `/Game/SH/DT_SH/ST_Ingredient` _value) (+ (`.Amount_32_E56828F94FB039E0485A0A9893929FEF` (break `/Game/SH/DT_SH/ST_Ingredient` _value)) 1)))
      (else
        (`BlueprintMapLibrary.Map_Add` (`local.PlateIngredient`) (`/Game/SH/Blueprint_SH/Ingredient/BP_Food_SH.FoodItemAsset`) (make `/Game/SH/DT_SH/ST_Ingredient` (`/Game/JH/Blueprints/Interactable/Grabbable/BP_Food_JH.State` (`local.FoodItems`)) 1)))))
  (return (`local.PlateIngredient`)))

(fn `UserConstructionScript`
  (`parent.UserConstructionScript`))