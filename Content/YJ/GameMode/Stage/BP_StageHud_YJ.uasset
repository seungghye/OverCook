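; BP_StageHud_YJ is the stage HUD, which creates the WBP_StageHudWidget_YJ widget and adds it to the viewport on BeginPlay.
; BindWidgets then casts the game state to BP_StageGameState_YJ and stores it, calling itself again immediately if the cast fails.
; The sequence after a successful cast is empty, and the left-time dispatcher binding is disconnected, so no widget binding actually runs.
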(event `self.ReceiveBeginPlay`
  (bind _returnvalue (`|CreateWidget` "/Game/YJ/Widget/Stage/WBP_StageHudWidget_YJ.WBP_StageHudWidget_YJ_C"))
  (bind _output_get (set `self.HudWidget` _returnvalue))
  (`UserWidget.AddToViewport` _output_get 0)
  (`self.BindWidgets`))

(fn `BindWidgets`
  (locals (StageGameState :type "/Game/YJ/GameMode/Stage/BP_StageGameState_YJ Object Reference"))
  (bind _asbp_stage_game_state_yj (cast `/Game/YJ/GameMode/Stage/BP_StageGameState_YJ` (`GameplayStatics.GetGameState`))
    (:`then`
      (set `local.StageGameState` _asbp_stage_game_state_yj)
      (`|ExecutionSequence`))
    (:`CastFailed`
      (`self.BindWidgets`))))

(fn `UserConstructionScript`)