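; Game mode for an Overcooked-style stage that runs the countdown and generates recipe orders.
; On BeginPlay it seeds the game state's time and score and takes the recipe menu from the game instance's selected stage.
; Looping timers decrease time and add random orders through the game state.
; Helpers add score and remove orders by matching class, while EndStage and SubmitFood are still empty stubs.
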(event `self.ReceiveBeginPlay`
  (`self.IntializeGameState`)
  (`self.StartStage`))

(fn `AddOrderedRecipe`
  (`/Game/YJ/GameMode/Stage/BP_StageGameState_YJ.ResAddOrderedRecipe` (`self.StageGameState`) (`KismetArrayLibrary.Array_Random` (`self.RecipeMenu`))))

(fn `AddScore`
  (params (InScore :type Integer))
  (`/Game/YJ/GameMode/Stage/BP_StageGameState_YJ.AddScore` (`self.StageGameState`) InScore))

(fn `DoStageTimer`
  (bind _stagegamestate (`self.StageGameState`))
  (`/Game/YJ/GameMode/Stage/BP_StageGameState_YJ.DecreaseLeftTime` _stagegamestate)
  (if (<= (`/Game/YJ/GameMode/Stage/BP_StageGameState_YJ.LeftTime` _stagegamestate) 0)
    (`self.EndStage`)))

(fn `EndStage`)

(fn `IntializeGameState`
  (bind _asbp_stage_game_state_yj (cast `/Game/YJ/GameMode/Stage/BP_StageGameState_YJ` (`GameplayStatics.GetGameState`))
    (:`then`
      (set `self.StageGameState` _asbp_stage_game_state_yj)
      (`|ExecutionSequence`
        (:`then_0`
          (set `/Game/YJ/GameMode/Stage/BP_StageGameState_YJ.LeftTime` (`self.InitialStageTime`) (`self.StageGameState`)))
        (:`then_1`
          (set `/Game/YJ/GameMode/Stage/BP_StageGameState_YJ.Score` (`self.InitialScore`) (`self.StageGameState`)))
        (:`then_2`
          (bind _asbp_over_cook_game_instance_yj (cast `/Game/YJ/GameMode/BP_OverCookGameInstance_YJ` (`GameplayStatics.GetGameInstance`)))
          (set `self.RecipeMenu` (`.RecipeMenu_20_7845BE26440E255B02BC25A61C5B85C2` (break `/Game/YJ/Data/Lobby/ST_StageInfo` (`/Game/YJ/GameMode/BP_OverCookGameInstance_YJ.SelectedStage` _asbp_over_cook_game_instance_yj)))))))
    (:`CastFailed`
      (`KismetSystemLibrary.PrintString` "GM: GameState cast failed" true true (struct :`R` 1.0 :`G` 0.263207 :`A` 1.0) 60.0))))

(fn `StartStage`
  (`KismetSystemLibrary.K2_SetTimer` null "DoStageTimer" 1.0 true)
  (`KismetSystemLibrary.K2_SetTimer` null "AddOrderedRecipe" 5.0 true))

(fn `SubmitFood`
  (params (SubmittedFood :type "/Game/SH/DT_SH/DA_Recipe_BP Object Reference"))
  ;[1 1 1] Merge후 DA_Recipe의 Score가져오기
)

(fn `SubtractOrderedRecipe`
  (params (PickedUpRecipe :type "/Game/SH/DT_SH/DA_Recipe_BP Object Reference"))
  (for (_array_element _array_index) (`/Game/YJ/GameMode/Stage/BP_StageGameState_YJ.OrderedRecipeList` (`self.StageGameState`))
    (if (== (`GameplayStatics.GetObjectClass` _array_element) (`GameplayStatics.GetObjectClass` PickedUpRecipe))
      (`/Game/YJ/GameMode/Stage/BP_StageGameState_YJ.SubtractOrderedRecipe` (`self.StageGameState`) _array_index)
      (return)))
  (return))

(fn `UserConstructionScript`)