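; Lobby player controller that blends its view to the lobby truck and has the authority side possess it.
; On BeginPlay it reads the truck and blend time from BP_LobbyGameMode_YJ, starts the camera blend, then possesses the truck after that delay on authority.
; On possession it sets game-only input and adds the lobby Enhanced Input mapping context, plus the truck context on authority only.
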(event `self.ReceivePossess`
  (params (PossessedPawn :type "Pawn Object Reference"))
  (`self.ResOnPossess`))

(event `ResOnPossess`
  (bind _returnvalue (subsystem `EnhancedInputLocalPlayerSubsystem`))
  (`WidgetBlueprintLibrary.SetInputMode_GameOnly` self)
  (`EnhancedInputSubsystemInterface.AddMappingContext` _returnvalue "/Game/YJ/Input/IMC_Lobby_YJ.IMC_Lobby_YJ" 0 (struct))
  (`/Engine/EditorBlueprintResources/ActorMacros.Switch Has Authority`
    (:`Authority`
      (`EnhancedInputSubsystemInterface.AddMappingContext` _returnvalue "/Game/YJ/Input/IMC_LobbyTruck_YJ.IMC_LobbyTruck_YJ" 0 (struct)))))

(event `self.ReceiveBeginPlay`
  (`|ExecutionSequence`
    (:`then_0`
      (bind _asbp_lobby_game_mode_yj (cast `/Game/YJ/GameMode/Lobby/BP_LobbyGameMode_YJ` (`GameplayStatics.GetGameMode`)))
      (bind _lobbytruck (`/Game/YJ/GameMode/Lobby/BP_LobbyGameMode_YJ.LobbyTruck` _asbp_lobby_game_mode_yj))
      (bind _blendtime (`/Game/YJ/GameMode/Lobby/BP_LobbyGameMode_YJ.BlendTime` _asbp_lobby_game_mode_yj))
      (`self.SetViewTargetWithBlend` _lobbytruck _blendtime))
    (:`then_1`
      (`/Engine/EditorBlueprintResources/ActorMacros.Switch Has Authority`
        (:`Authority`
          (`KismetSystemLibrary.Delay` _blendtime)
          (`self.Possess` _lobbytruck))))))

(fn `UserConstructionScript`)