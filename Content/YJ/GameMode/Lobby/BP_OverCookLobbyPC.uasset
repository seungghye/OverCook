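; Lobby player controller for the Overcook game, where the host drives a shared truck to pick a stage.
; On BeginPlay it blends the view to the game mode's LobbyTruck, and the authority side possesses it after the blend.
; Possession adds lobby input mappings, with truck controls only for authority.
; The open-level input checks for an overlapping BP_Stage at the pawn, then server-travels to the hardcoded YJLevel.
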(event `self.ReceivePossess`
  (params (PossessedPawn :type "Pawn Object Reference"))
  (`self.ResOnPossess`))

(event `ResOnPossess`
  (bind _returnvalue (subsystem `EnhancedInputLocalPlayerSubsystem`))
  (`/Engine/EditorBlueprintResources/ActorMacros.Switch Has Authority`
    (:`Authority`
      (`EnhancedInputSubsystemInterface.AddMappingContext` _returnvalue "/Game/YJ/Input/IMC_LobbyTruck_YJ.IMC_LobbyTruck_YJ" 0 (struct))
      (`EnhancedInputSubsystemInterface.AddMappingContext` _returnvalue "/Game/YJ/Input/IMC_Lobby_YJ.IMC_Lobby_YJ" 0 (struct)))
    (:`Remote`
      (`EnhancedInputSubsystemInterface.AddMappingContext` _returnvalue "/Game/YJ/Input/IMC_Lobby_YJ.IMC_Lobby_YJ" 0 (struct)))))

(event `self.ReceiveBeginPlay`
  (`|ExecutionSequence`
    (:`then_0`
      (bind _asbp_over_cook_lobby_game_mode_yj (cast `/Game/YJ/GameMode/Lobby/BP_OverCookLobbyGameMode_YJ` (`GameplayStatics.GetGameMode`)))
      (bind _lobbytruck (`/Game/YJ/GameMode/Lobby/BP_OverCookLobbyGameMode_YJ.LobbyTruck` _asbp_over_cook_lobby_game_mode_yj))
      (bind _blendtime (`/Game/YJ/GameMode/Lobby/BP_OverCookLobbyGameMode_YJ.BlendTime` _asbp_over_cook_lobby_game_mode_yj))
      (`self.SetViewTargetWithBlend` _lobbytruck _blendtime))
    (:`then_1`
      (`/Engine/EditorBlueprintResources/ActorMacros.Switch Has Authority`
        (:`Authority`
          (`KismetSystemLibrary.Delay` _blendtime)
          (`self.Possess` _lobbytruck))))))

(event `EnhancedInput|/Game/YJ/Input/IA_OpenLevel`
  (params (ActionValue :type Boolean) (ElapsedSeconds :type "Float (double-precision)") (TriggeredSeconds :type "Float (double-precision)") (InputAction :type "InputAction Object Reference" :default "/Game/YJ/Input/IA_OpenLevel.IA_OpenLevel"))
  (:`Triggered`
    (bind _outactors (`KismetSystemLibrary.BoxOverlapActors` :`BoxPos` (`self.K2_GetActorLocation` (`self.K2_GetPawn`)) :`ActorClassFilter` "/Game/YJ/Blueprints/Lobby/BP_Stage.BP_Stage_C"))
    (`/Engine/EditorBlueprintResources/StandardMacros.IsValid` (`|GetArrayItem` _outactors)
      (:`Is Valid`
        ;[1 1 1] 이동할 '맵 이름' 주의
        (`KismetSystemLibrary.PrintString` "Run ExecuteConsoleCommand !" true true (struct :`R` 1.0 :`B` 0.884576 :`A` 1.0) 60.0)
        (`KismetSystemLibrary.ExecuteConsoleCommand` "servertravel YJLevel" null)))))

(fn `UserConstructionScript`)