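; Lobby HUD that shows the lobby widget and relays chat between it and the rest of the game.
; On BeginPlay it creates WBP_LobbyHudWidget_YJ and binds a handler to its chat box's text-commit event.
; Committed text is broadcast through the ChatCommitted dispatcher with the user name from the game instance.
; AddChat passes incoming messages to the widget for display.
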(event `self.ReceiveBeginPlay`
  (bind _returnvalue (`|CreateWidget` "/Game/YJ/Widget/Lobby/WBP_LobbyHudWidget_YJ.WBP_LobbyHudWidget_YJ_C"))
  (bind _output_get (set `self.HudWidget` _returnvalue))
  (`UserWidget.AddToViewport` _output_get 0)
  (`self.BindWidgets`))

(fn `AddChat`
  (params (UserName :type String) (Chat :type Text))
  (`/Game/YJ/Widget/Lobby/WBP_LobbyHudWidget_YJ.AddChat` (`self.HudWidget`) UserName Chat))

(fn `BindWidgets`
  (`|ExecutionSequence`
    (:`then_0`
      (add `EditableText.OnTextCommitted` (`/Game/YJ/Widget/Lobby/WBP_LobbyHudWidget_YJ.EditableText_ChatBox` (`self.HudWidget`)) (`|CreateDelegate` :!event `EventTextCommitted`)))))

(fn `EventTextCommitted`
  (params (Text :type "Text (by ref)") (CommitMethod :type "ETextCommit Enum" :default "Default"))
  (bind _asbp_over_cook_game_instance_yj (cast `/Game/YJ/GameMode/BP_OverCookGameInstance_YJ` (`GameplayStatics.GetGameInstance`))
    (:`then`
      (`self.EventDispatcher_ChatCommitted` (`/Game/YJ/GameMode/BP_OverCookGameInstance_YJ.UserName` _asbp_over_cook_game_instance_yj) Text)
      (return))
    (:`CastFailed`
      (`KismetSystemLibrary.PrintString` "LobbyHud : GameInstance CastFailed" true true (struct :`G` 0.66 :`B` 1.0 :`A` 1.0) 60.0))))

(fn `UserConstructionScript`)