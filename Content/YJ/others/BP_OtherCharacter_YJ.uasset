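; Player character for a cooking game that moves, grabs and drops objects, and starts or stops cooking interactions.
; Input passes through paired Req/Res events to short forward sphere traces on separate grab and cooking channels, which send messages to hit actors.
; Grabbed objects attach to the Hands component; a missed grab trace drops the held object when ObjectPlace is valid.
; SetIsCooking stores the interacting object and toggles an extra Enhanced Input mapping context.
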(event `EnhancedInput|/Game/JH/Input/IA_Move_JH`
  (params (ActionValue :type "Vector2D Structure") (ElapsedSeconds :type "Float (double-precision)") (TriggeredSeconds :type "Float (double-precision)") (InputAction :type "InputAction Object Reference" :default "/Game/JH/Input/IA_Move_JH.IA_Move_JH"))
  ;[1 1 1] 캐릭터 기본 움직임
  (:`Triggered`
    (`self.AddMovementInput` (`KismetMathLibrary.Conv_Vector2DToVector` ActionValue))))

(event `EnhancedInput|/Game/JH/Input/IA_Grab_JH`
  (params (ActionValue :type Boolean) (ElapsedSeconds :type "Float (double-precision)") (TriggeredSeconds :type "Float (double-precision)") (InputAction :type "InputAction Object Reference" :default "/Game/JH/Input/IA_Grab_JH.IA_Grab_JH"))
  ;[1 1 1] 상호작용(스페이스바)으로 개체 그랩
  (:`Started`
    (`self.ReqGrabAndDrop`)))

(event `ReqGrabAndDrop`
  ;[1 1 1] 상호작용(스페이스바)으로 개체 그랩
  (`self.ResGrabAndDrop`))

(event `ResGrabAndDrop`
  (bind (_isgetgrabbedobject _grabbedobject) (`self.Get Grabbed Object`))
  ;[1 1 1] 상호작용(스페이스바)으로 개체 그랩
  (bind (_returnvalue _outhit) (`self.GrabAndDrop` "TraceTypeQuery3"))
  (if _returnvalue
    (message `/Game/JH/Blueprints/Data/BPI_Interactable_JH.Grab` (`.HitActor` (`GameplayStatics.BreakHitResult` _outhit)) self)
    (elif _isgetgrabbedobject
      (if (`KismetSystemLibrary.IsValid` (`self.ObjectPlace`))
        (`/Game/JH/Blueprints/Interactable/BP_Grabbable_JH.Drop` _grabbedobject)
        (set `self.GrabbedObject` null)))))

(event `Grab`
  (params (ObjectToGrab :type "/Game/JH/Blueprints/Interactable/BP_Grabbable_JH Object Reference"))
  (bind _output_get (set `self.GrabbedObject` ObjectToGrab))
  (`self.K2_AttachToComponent` _output_get (`self.Hands`) "None" "KeepWorld" "KeepWorld" "KeepWorld" true)
  (`KismetSystemLibrary.MoveComponentTo` (`Actor.RootComponent` (`self.GrabbedObject`))))

(event `EnhancedInput|/Game/JH/Input/IA_Cooking_JH`
  (params (ActionValue :type Boolean) (ElapsedSeconds :type "Float (double-precision)") (TriggeredSeconds :type "Float (double-precision)") (InputAction :type "InputAction Object Reference" :default "/Game/JH/Input/IA_Cooking_JH.IA_Cooking_JH"))
  (:`Started`
    (if (not (`self.IsCooking`))
      (`self.ReqCooking`)))
  (:`Completed`
    (if (`self.IsCooking`)
      (`self.ReqStopCooking`))))

(event `ResCooking`
  (bind (_returnvalue _outhit) (`self.GrabAndDrop` "TraceTypeQuery4"))
  (if _returnvalue
    (message `/Game/JH/Blueprints/Data/BPI_Interactable_JH.Cooking` (`.HitActor` (`GameplayStatics.BreakHitResult` _outhit)) self)))

(event `ReqCooking`
  (`self.ResCooking`))

(event `EnhancedInput|/Game/JH/Input/IA_StopInteraction_JH`
  (params (ActionValue :type Boolean) (ElapsedSeconds :type "Float (double-precision)") (TriggeredSeconds :type "Float (double-precision)") (InputAction :type "InputAction Object Reference" :default "/Game/JH/Input/IA_StopInteraction_JH.IA_StopInteraction_JH"))
  (:`Started`
    (`self.ReqStopCooking`)))

(event `ResStopCooking`
  (`self.StopCooking`))

(event `StopCooking`
  (`/Game/JH/Blueprints/Data/BPI_Interactable_JH.StopCooking` (`self.InteractingObject`)))

(event `ReqStopCooking`
  (`self.ResStopCooking`))

(event `SetIsCooking`
  (params (IsCooking :type Boolean) (InteractingObject :type "/Game/JH/Blueprints/Data/BPI_Interactable_JH Interface"))
  (bind _returnvalue (pcsubsystem `EnhancedInputLocalPlayerSubsystem` (`GameplayStatics.GetPlayerController` 0)))
  (set `self.IsCooking` IsCooking)
  (set `self.InteractingObject` InteractingObject)
  (if (`self.IsCooking`)
    (`EnhancedInputSubsystemInterface.AddMappingContext` _returnvalue "/Game/JH/Input/IMC_Interacting_JH.IMC_Interacting_JH" 0 (struct))
    (else
      (`EnhancedInputSubsystemInterface.RemoveMappingContext` _returnvalue "/Game/JH/Input/IMC_Interacting_JH.IMC_Interacting_JH" (struct)))))

(fn `Get Grabbed Object`
  (returns (IsGetGrabbedObject :type Boolean) (GrabbedObject :type "/Game/JH/Blueprints/Interactable/BP_Grabbable_JH Object Reference"))
  (bind _grabbedobject (`self.GrabbedObject`))
  (return (`KismetSystemLibrary.IsValid` _grabbedobject) _grabbedobject))

(fn `GrabAndDrop`
  (params (TraceChannel :type "ETraceTypeQuery Enum" :default "TraceTypeQuery1"))
  (returns (ReturnValue :type Boolean) (OutHit :type "HitResult Structure"))
  (bind _x (.x (+ (* (`self.GetActorForwardVector`) 50.0) (`self.K2_GetActorLocation`))))
  (bind _y (.y (+ (* (`self.GetActorForwardVector`) 50.0) (`self.K2_GetActorLocation`))))
  (bind _z (.z (+ (* (`self.GetActorForwardVector`) 50.0) (`self.K2_GetActorLocation`))))
  (bind (_outhit _returnvalue) (`KismetSystemLibrary.SphereTraceSingle` (`KismetMathLibrary.MakeVector` _x _y (+ _z -50.0)) (`KismetMathLibrary.MakeVector` _x _y (+ _z 10.0)) 30.0 TraceChannel false (`|MakeArray` (`self.GrabbedObject`) :!type "Actor Object Reference")))
  (return _returnvalue _outhit))

(fn `UserConstructionScript`)