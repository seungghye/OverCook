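; Food dispenser table interactable that hands players a new food item defined by its FoodItemAsset.
; On Grab/Drop it defers to the parent table logic when a grabbable placed object exists, or when the table is empty and the player holds something.
; An empty-handed player at an empty table gets a spawned BP_Food_JH flagged as sliced, grabbed immediately.
; The construction script applies the asset's Icon as material on Cube and SMBottom.
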(event `self.Grab/Drop`
  (params (Player :type "/Game/Common/GameMode/Stage/BP_Character_JH Object Reference"))
  (bind _placeobject (`self.PlaceObject`)
    (:`then`
      (if (`/Game/Common/Blueprint/Interactable/Grabbable/BP_Grabbable_JH.CanBeGrabbed` _placeobject Player)
        (`parent.Grab/Drop` Player :!label _label)))
    (:`else`
      (if (`/Game/Common/GameMode/Stage/BP_Character_JH.Get Grabbed Object` Player)
        (goto _label)
        (else
          ;[1 1 1] 병합 후 FoodItemAsset 연결해주세요.
          (bind _returnvalue (`|SpawnActorFromClass` "/Game/Common/Blueprint/Interactable/Grabbable/BP_Food_JH.BP_Food_JH_C" (`self.GetTransform`) "Undefined" "MultiplyWithRoot" null true (`self.FoodItemAsset`) null))
          (`/Game/Common/Data/BPI_Interactable_JH.Grab/Drop` _returnvalue Player))))))

(fn `UserConstructionScript`
  (`parent.UserConstructionScript`)
  (`KismetMaterialLibrary.CreateDynamicMaterialInstance` "/Game/Common/Asset/kitchen_Tools/Material/M_DarwerTomato.M_DarwerTomato")
  (`PrimitiveComponent.SetMaterial` (`self.Cube`) 0 (`/Game/Common/Data/FoodItem/DA_Food_Item_BP.Icon` (`self.FoodItemAsset`)))
  (`PrimitiveComponent.SetMaterial` (`self.SM_Bottom`) 0 (`/Game/Common/Data/FoodItem/DA_Food_Item_BP.Icon` (`self.FoodItemAsset`))))