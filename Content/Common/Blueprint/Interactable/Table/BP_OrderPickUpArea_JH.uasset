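; BP_OrderPickUpArea_JH is an interactable order pick-up area where the player hands in plated food.
; On Grab/Drop, a held non-empty plate has its ingredients compared to a test recipe, with the result only printed.
; The plate is then destroyed, the player's grab reference cleared, and a plate added back to a plate box.
; That box is the assigned PlateBox, otherwise a random one from those gathered at BeginPlay.
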(event `self.ReceiveBeginPlay`
  (`self.PlateBox`
    (:`then`)
    (:`else`
      (bind _outactors (`GameplayStatics.GetAllActorsOfClass` "/Game/Common/Blueprint/Interactable/Table/BP_PlateBox_JH.BP_PlateBox_JH_C"))
      (set `self.AllPlateBoxes` _outactors))))

(event `/Game/Common/Data/BPI_Interactable_JH.Grab/Drop`
  (params (Player :type "/Game/Common/GameMode/Stage/BP_Character_JH Object Reference"))
  (bind _asbp_plate_sh (cast `/Game/Common/Blueprint/Interactable/Grabbable/BP_Plate_SH` (`.GrabbedObject` (`/Game/Common/GameMode/Stage/BP_Character_JH.Get Grabbed Object` Player))))
  (if (not (`/Game/Common/Blueprint/Interactable/Grabbable/BP_Kitchenware_JH.IsEmpty` _asbp_plate_sh))
    (`KismetSystemLibrary.PrintString` (`KismetStringLibrary.Conv_BoolToString` (`/Game/Common/Data/Recipe/DA_Recipe_BP.Compare` (`self.RecipeForTest`) (`/Game/Common/Blueprint/Interactable/Grabbable/BP_Plate_SH.GetIngredients` _asbp_plate_sh))))
    (`self.K2_DestroyActor` _asbp_plate_sh)
    (set `/Game/Common/GameMode/Stage/BP_Character_JH.GrabbedObject` null Player)
    (`/Game/Common/Blueprint/Interactable/Table/BP_PlateBox_JH.AddPlate` (`self.GetCurPlateBox`))))

(fn `GetCurPlateBox`
  (returns (PlateBox :type "/Game/Common/Blueprint/Interactable/Table/BP_PlateBox_JH Object Reference"))
  (bind _platebox (`self.PlateBox`)
    (:`then`
      (return _platebox))
    (:`else`
      (return (`KismetArrayLibrary.Array_Random` (`self.AllPlateBoxes`))))))

(fn `UserConstructionScript`)