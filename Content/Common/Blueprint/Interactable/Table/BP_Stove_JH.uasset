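; BP_Stove_JH is an interactable stove table that starts with cookware on it and toggles that object's cooking state.
; On BeginPlay it spawns a BP_Cookware_JH at the ObjectPlace component, removes its physics, stores it as PlaceObject and attaches it.
; Grab and Place extend the parent's logic, sending CookMessage false before an object is taken and true after one is placed.
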(event `self.ReceiveBeginPlay`
  (`self.InitCookware`))

(event `self.Grab`
  (params (Player :type "/Game/Common/GameMode/Stage/BP_Character_JH Object Reference"))
  (message `/Game/Common/Data/BPI_Cookware.Cook` (`self.PlaceObject`) false)
  (`parent.Grab` Player))

(event `self.Place`
  (params (ObjectToPlace :type "/Game/Common/Blueprint/Interactable/Grabbable/BP_Grabbable_JH Object Reference") (Player :type "/Game/Common/GameMode/Stage/BP_Character_JH Object Reference"))
  (if true
    (`parent.Place` ObjectToPlace Player)
    (message `/Game/Common/Data/BPI_Cookware.Cook` (`self.PlaceObject`) true)))

(fn `InitCookware`
  (bind _returnvalue (`|SpawnActorFromClass` "/Game/Common/Blueprint/Interactable/Grabbable/BP_Cookware_JH.BP_Cookware_JH_C" (`KismetMathLibrary.MakeTransform` (`SceneComponent.K2_GetComponentLocation` (`self.ObjectPlace`))) "Undefined" "MultiplyWithRoot" null null))
  (`/Game/Common/Blueprint/Interactable/Grabbable/BP_Grabbable_JH.RemovePhysics` _returnvalue)
  (set `self.PlaceObject` _returnvalue)
  (`self.K2_AttachToComponent` _returnvalue (`self.ObjectPlace`) "None" "KeepWorld" "KeepWorld" "KeepWorld" true))

(fn `UserConstructionScript`
  (`parent.UserConstructionScript`))