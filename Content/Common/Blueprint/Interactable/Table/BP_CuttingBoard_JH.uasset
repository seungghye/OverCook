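; Cutting board interactable where a player slices a placed food item over time in a cooking game.
; Cooking starts only on sliceable food, then Tick advances progress at constant speed, driving a progress-bar widget and Niagara effect.
; At full progress it updates the food's state and releases the player.
; Grab/drop works only at zero or full progress and resets it; a helper sphere-traces in front of the board, ignoring the plate.
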(event `self.ReceiveBeginPlay`
  (`SceneComponent.SetVisibility` (`self.Widget`) false false)
  (`ActorComponent.Deactivate` (`self.Niagara`)))

(event `self.ReceiveTick`
  (params (DeltaSeconds :type "Float (single-precision)"))
  (`parent.ReceiveTick` DeltaSeconds)
  (if (`self.IsInteracting`)
    (`SceneComponent.SetVisibility` (`self.Widget`) true false)
    (`self.SetProgress` DeltaSeconds)
    (if (== (`self.Progress`) 1.0)
      (`/Game/Common/Data/BPI_Interactable_JH.StopCooking`)
      (bind _asbp_food_jh (cast `/Game/Common/Blueprint/Interactable/Grabbable/BP_Food_JH` (`self.PlaceObject`)))
      (`/Game/Common/Blueprint/Interactable/Grabbable/BP_Food_JH.SetState` _asbp_food_jh "NewEnumerator1")
      (`SceneComponent.SetVisibility` (`self.Widget`) false false))))

(event `/Game/Common/Data/BPI_Interactable_JH.Grab/Drop`
  (params (Player :type "/Game/Common/GameMode/Stage/BP_Character_JH Object Reference"))
  (if (`self.CanGrabObject`)
    (`parent.Grab/Drop` Player)
    (set `self.Progress` 0.0)))

(event `/Game/Common/Data/BPI_Interactable_JH.Cooking`
  (params (Player :type "/Game/Common/GameMode/Stage/BP_Character_JH Object Reference"))
  (bind _asbp_food_jh (cast `/Game/Common/Blueprint/Interactable/Grabbable/BP_Food_JH` (`self.PlaceObject`)))
  (if (`/Game/Common/Blueprint/Interactable/Grabbable/BP_Food_JH.IsCanSlice` _asbp_food_jh)
    (`/Game/Common/Blueprint/Interactable/Grabbable/BP_Food_JH.SetState` _asbp_food_jh "NewEnumerator0")
    (`/Game/Common/GameMode/Stage/BP_Character_JH.SetIsCooking` Player true self)
    (set `self.InteractingPlayer` Player)
    (set `self.IsInteracting` true)))

(event `/Game/Common/Data/BPI_Interactable_JH.StopCooking`
  (set `self.IsInteracting` false)
  (`/Game/Common/GameMode/Stage/BP_Character_JH.SetIsCooking` (`self.InteractingPlayer`) false null)
  (`ActorComponent.Deactivate` (`self.Niagara`)))

(fn `CanGrabObject`
  (returns (ReturnValue :type Boolean))
  (return (or (== (`self.Progress`) 0.0) (== (`self.Progress`) 1.0))))

(fn `CheckForPlateOverlap`
  (params (InputPin :type "ETraceTypeQuery Enum" :default "TraceTypeQuery1"))
  (returns (ReturnValue :type Boolean))
  (bind _x (.x (+ (`self.GetActorForwardVector`) (`self.K2_GetActorLocation`))))
  (bind _y (.y (+ (`self.GetActorForwardVector`) (`self.K2_GetActorLocation`))))
  (bind _z (.z (+ (`self.GetActorForwardVector`) (`self.K2_GetActorLocation`))))
  (bind (_outhit _returnvalue) (`KismetSystemLibrary.SphereTraceSingle` (`KismetMathLibrary.MakeVector` _x _y (+ _z -80.0)) (`KismetMathLibrary.MakeVector` _x _y (+ _z 20.0)) 30.0 InputPin false (`|MakeArray` (`self.Plate`) :!type "Actor Object Reference")))
  (return _returnvalue))

(fn `SetProgress`
  (params (DeltaSeconds :type "Float (single-precision)"))
  (bind _output_get (set `self.Progress` (`KismetMathLibrary.FInterpTo_Constant` (`self.Progress`) 1.0 DeltaSeconds (`self.SlicingSpeed`))))
  (bind _aswbp_progress_bar_jh (cast `/Game/Common/Widget/Stage/WBP_ProgressBar_JH` (`WidgetComponent.GetUserWidgetObject` (`self.Widget`))))
  (`/Game/Common/Widget/Stage/WBP_ProgressBar_JH.SetProgress` _aswbp_progress_bar_jh _output_get)
  (`KismetSystemLibrary.PrintString` (`KismetStringLibrary.Conv_DoubleToString` _output_get) true true (struct :`G` 0.66 :`B` 1.0 :`A` 1.0) DeltaSeconds)
  (`ActorComponent.Activate` (`self.Niagara`) false))

(fn `UserConstructionScript`
  (`parent.UserConstructionScript`))