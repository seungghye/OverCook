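; Entry-panel Blueprint that hosts the create-session widget through its Widget component.
; On BeginPlay it passes CreatingLevelName, the lobby map to create, into WBP_CreateSessionWidget_YJ as NextLevelName.
; It then binds an event to the widget's cancel-click dispatcher; the handler's behavior is not shown.
; Both setup functions cast the component's user widget and do nothing if the cast fails.
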(event `self.ReceiveBeginPlay`
  ;[1 1 1] 생성할 로비맵 이름 주의
  (`self.InitializeWidget` (`self.CreatingLevelName`))
  (`self.BindWidget`))

(fn `BindWidget`
  (bind _aswbp_create_session_widget_yj (cast `/Game/Common/Widget/Entry/WBP_CreateSessionWidget_YJ` (`WidgetComponent.GetUserWidgetObject` (`self.Widget`))))
  (add `/Game/Common/Widget/Entry/WBP_CreateSessionWidget_YJ.EventDispatcher_ClickCancel` _aswbp_create_session_widget_yj (`|CreateDelegate` :!event `SetViewTarget`)))

(fn `InitializeWidget`
  (params (NextLevelName :type Name))
  (bind _aswbp_create_session_widget_yj (cast `/Game/Common/Widget/Entry/WBP_CreateSessionWidget_YJ` (`WidgetComponent.GetUserWidgetObject` (`self.Widget`))))
  (set `/Game/Common/Widget/Entry/WBP_CreateSessionWidget_YJ.NextLevelName` NextLevelName _aswbp_create_session_widget_yj))

(fn `UserConstructionScript`)