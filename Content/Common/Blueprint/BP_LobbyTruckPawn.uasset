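; Player-driven truck pawn for the lobby, used to move around and enter stages.
; Enhanced Input move action feeds world-space movement input and eases the truck's rotation toward the input direction with a fixed-alpha lerp.
; The open-level action runs a box overlap around the truck for BP_LobbyStageSelector actors and calls TravelStage on the first hit, otherwise printing a debug message.
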(event `EnhancedInput|/Game/Common/Input/Lobby/IA_Move_YJ`
  (params (ActionValue :type "Vector2D Structure") (ElapsedSeconds :type "Float (double-precision)") (TriggeredSeconds :type "Float (double-precision)") (InputAction :type "InputAction Object Reference" :default "/Game/Common/Input/Lobby/IA_Move_YJ.IA_Move_YJ"))
  (bind _returnvalue (`KismetMathLibrary.Conv_Vector2DToVector` ActionValue))
  (:`Triggered`
    (`self.AddMovementInput` _returnvalue)
    (`self.K2_SetActorRotation` (`KismetMathLibrary.RLerp` (`self.K2_GetActorRotation`) (`KismetMathLibrary.Conv_VectorToRotator` _returnvalue) 0.1 true))))

(event `EnhancedInput|/Game/Common/Input/Lobby/IA_OpenLevel_YJ`
  (params (ActionValue :type Boolean) (ElapsedSeconds :type "Float (double-precision)") (TriggeredSeconds :type "Float (double-precision)") (InputAction :type "InputAction Object Reference" :default "/Game/Common/Input/Lobby/IA_OpenLevel_YJ.IA_OpenLevel_YJ"))
  (:`Started`
    ;[1 1 1] BoxExtent 크기 설정
    (bind _outactors (`KismetSystemLibrary.BoxOverlapActors` (`self.K2_GetActorLocation`) (100.0 100.0 100.0) (`|MakeArray` "ObjectTypeQuery1" "ObjectTypeQuery2" "ObjectTypeQuery3" "ObjectTypeQuery4" "ObjectTypeQuery5" "ObjectTypeQuery6" :!type "EObjectTypeQuery Enum") "/Game/Common/Blueprint/BP_LobbyStageSelector.BP_LobbyStageSelector_C"))
    (bind _output (`|GetArrayItem` _outactors))
    (`/Engine/EditorBlueprintResources/StandardMacros.IsValid` _output
      (:`Is Valid`
        (bind _asbp_lobby_stage_selector (cast `/Game/Common/Blueprint/BP_LobbyStageSelector` _output))
        (`/Game/Common/Blueprint/BP_LobbyStageSelector.TravelStage` _asbp_lobby_stage_selector))
      (:`Is Not Valid`
        (`KismetSystemLibrary.PrintString` "Truck: Overlaped Stage is NotValid")))))

(fn `UserConstructionScript`)