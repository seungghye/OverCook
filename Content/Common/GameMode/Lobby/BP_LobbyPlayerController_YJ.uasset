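; Lobby player controller that handles input setup, user registration and chat for an Overcooked-style game.
; On possess it adds the lobby mapping context, plus the truck context on authority, then passes the GameInstance user name to the lobby GameMode's user list.
; BindHud retries on a timer until the HUD exists, then binds its chat dispatcher.
; Chat uses a Req/Res pair, relaying messages through every lobby controller to its HUD.
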(event `self.ReceivePossess`
  (params (PossessedPawn :type "Pawn Object Reference"))
  ;[1 1 1] Possess하면 GameMode를 통해Possess캐릭터 설정과 GameState의 UserList 추가
  (`parent.ReceivePossess` PossessedPawn)
  (`KismetSystemLibrary.PrintString` (`KismetStringLibrary.Concat_StrStr` (`KismetSystemLibrary.GetDisplayName` PossessedPawn) " - On Possess") true true (struct :`R` 1.0 :`B` 0.670606 :`A` 1.0) 60.0)
  (`self.ResOnPossess` PossessedPawn))

(event `ResOnPossess`
  (params (PossessedPawn :type "Pawn Object Reference"))
  (bind _returnvalue (subsystem `EnhancedInputLocalPlayerSubsystem`))
  ;[1 1 1] Possess하면 GameMode를 통해Possess캐릭터 설정과 GameState의 UserList 추가
  (`KismetSystemLibrary.PrintString` "PC: ResOnPossess Called" true true (struct :`G` 0.66 :`B` 1.0 :`A` 1.0) 60.0)
  (`|ExecutionSequence`
    (:`then_0`
      (`WidgetBlueprintLibrary.SetInputMode_GameOnly` self)
      (`EnhancedInputSubsystemInterface.AddMappingContext` _returnvalue "/Game/Common/Input/Lobby/IMC_Lobby_YJ.IMC_Lobby_YJ" 0 (struct))
      (`/Engine/EditorBlueprintResources/ActorMacros.Switch Has Authority`
        (:`Authority`
          (`EnhancedInputSubsystemInterface.AddMappingContext` _returnvalue "/Game/Common/Input/Lobby/IMC_LobbyTruck_YJ.IMC_LobbyTruck_YJ" 0 (struct)))))
    (:`then_1`
      (bind _asbp_over_cook_game_instance_yj (cast `/Game/Common/GameMode/BP_OverCookGameInstance_YJ` (`GameplayStatics.GetGameInstance`))
        (:`then`
          (`KismetSystemLibrary.PrintString` "PC : Call ReqUserLogin" true true (struct :`G` 0.66 :`B` 1.0 :`A` 1.0) 60.0)
          (`self.ReqUserLogin` (`/Game/Common/GameMode/BP_OverCookGameInstance_YJ.UserName` _asbp_over_cook_game_instance_yj)))
        (:`CastFailed`
          (`KismetSystemLibrary.PrintString` "PC : GameInstance cast failed" true true (struct :`G` 0.66 :`B` 1.0 :`A` 1.0) 60.0))))))

(event `ReqUserLogin`
  (params (NewUserName :type String))
  ;[1 1 1] Possess하면 GameMode를 통해Possess캐릭터 설정과 GameState의 UserList 추가
  (bind _asbp_lobby_game_mode_yj (cast `/Game/Common/GameMode/Lobby/BP_LobbyGameMode_YJ` (`GameplayStatics.GetGameMode`)))
  (`KismetSystemLibrary.PrintString` "PC: Add User List Call" true true (struct :`G` 0.66 :`B` 1.0 :`A` 1.0) 60.0)
  (`/Game/Common/GameMode/Lobby/BP_LobbyGameMode_YJ.AddUserList` _asbp_lobby_game_mode_yj NewUserName self))

(event `self.ReceiveBeginPlay`
  (set `self.bShowMouseCursor` true)
  (`self.BindHud`))

(event `ReqChatCommitted`
  (params (UserName :type String) (Chat :type Text))
  ;[1 1 1] Chat System
  ;;[1 1 1] BindHud를 통해 Hud의 델리게이트로 인해 호출
  (bind _outactors (`GameplayStatics.GetAllActorsOfClass` "BP_LobbyPlayerController_YJ_C"))
  (for _array_element _outactors
    (`self.ResChatCommitted` _array_element UserName Chat)))

(event `ResChatCommitted`
  (params (UserName :type String) (Chat :type Text))
  ;[1 1 1] Chat System
  (bind _asbp_lobby_hud_yj (cast `/Game/Common/GameMode/Lobby/BP_LobbyHud_YJ` (`self.GetHUD`)))
  (`/Game/Common/GameMode/Lobby/BP_LobbyHud_YJ.AddChat` _asbp_lobby_hud_yj UserName Chat))

(fn `BindHud`
  (if (== (`GameplayStatics.GetPlayerController` 0) self)
    (bind _asbp_lobby_hud_yj (cast `/Game/Common/GameMode/Lobby/BP_LobbyHud_YJ` (`self.GetHUD`))
      (:`then`
        (`|ExecutionSequence`
          (:`then_0`
            (add `/Game/Common/GameMode/Lobby/BP_LobbyHud_YJ.EventDispatcher_ChatCommitted` _asbp_lobby_hud_yj (`|CreateDelegate` :!event `ReqChatCommitted`)))))
      (:`CastFailed`
        (`KismetSystemLibrary.K2_SetTimer` null "BindHud" 0.01)))))

(fn `UserConstructionScript`)