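; Lobby GameMode that registers players in the GameState user list and sets the default pawn: truck for the host, lobby pawn for clients.
; AddUserList fills the first slot without a valid controller, triggers a session update, and manually fires the list dispatcher because OnRep skips the server.
; UpdateSessionUserList writes names into session extra settings as 1-based "UserN" keys, preserving the other settings.
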(event `UpdateSessionUserList`
  ;[1 1 1] UpdateSession이 함수에 들어가지 못해 Event로 작성
  (bind (_numconnections _numprivateconnections _bislan _bisdedicated _ballowinvites _ballowjoininprogress _bisanticheatenabled _builduniqueid _extrasettings) (`AdvancedSessionsLibrary.GetSessionSettings`)
    (:`OnSuccess`
      (bind _asbp_lobby_game_state_yj (cast `/Game/Common/GameMode/Lobby/BP_LobbyGameState_YJ` (`GameplayStatics.GetGameState`)))
      (for (_array_element _array_index) (`/Game/Common/GameMode/Lobby/BP_LobbyGameState_YJ.UserList` _asbp_lobby_game_state_yj)
        (`KismetArrayLibrary.Array_Add` (`self.ModifiedExtraSettings`) (`AdvancedSessionsLibrary.MakeLiteralSessionPropertyString` (`KismetStringLibrary.Conv_StringToName` (`KismetStringLibrary.Concat_StrStr` "User" (`KismetStringLibrary.Conv_IntToString` (+ _array_index 1)))) (`.UserName_5_8C9B1B464DEEC796E8C5F4B44CBE680E` (break `/Game/Common/Data/LobbyData/ST_UserList` _array_element)))))
      (bind _modifiedsettingsarray (`AdvancedSessionsLibrary.AddOrModifyExtraSettings` _extrasettings (`self.ModifiedExtraSettings`)))
      (`UpdateSessionCallbackProxyAdvanced.UpdateSession` _modifiedsettingsarray _numconnections _numprivateconnections _bislan _ballowinvites _ballowjoininprogress true _bisdedicated
        (:`OnSuccess`
          (`KismetSystemLibrary.PrintString` "LobbyGM: Update Session Success!" true true (struct :`G` 0.66 :`B` 1.0 :`A` 1.0) 60.0))
        (:`OnFailure`
          (`KismetSystemLibrary.PrintString` "LobbyGM: Update Session Failed" true true (struct :`G` 0.66 :`B` 1.0 :`A` 1.0) 60.0))))))

(event `self.K2_PostLogin`
  (params (NewPlayer :type "PlayerController Object Reference"))
  ;[1 1 1] Set Default Pawn Class (Server=Truck / Client=LobbyPawn)
  (`parent.K2_PostLogin` NewPlayer)
  (if (== NewPlayer (`GameplayStatics.GetPlayerController` 0))
    (set `self.DefaultPawnClass` "/Game/Common/Blueprint/BP_LobbyTruckPawn.BP_LobbyTruckPawn_C")
    (else
      (set `self.DefaultPawnClass` "/Game/Common/GameMode/Lobby/BP_LobbyPawn_YJ.BP_LobbyPawn_YJ_C"))))

(fn `AddUserList`
  (params (NewUserName :type "String (by ref)") (NewUserController :type "PlayerController Object Reference"))
  (locals (GameState :type "/Game/Common/GameMode/Lobby/BP_LobbyGameState_YJ Object Reference"))
  (bind _asbp_lobby_game_state_yj (cast `/Game/Common/GameMode/Lobby/BP_LobbyGameState_YJ` (`GameplayStatics.GetGameState`))
    (:`then`
      (set `local.GameState` _asbp_lobby_game_state_yj)
      (bind _userlist (`/Game/Common/GameMode/Lobby/BP_LobbyGameState_YJ.UserList` _asbp_lobby_game_state_yj))
      (for (_array_element _array_index) _userlist
        (`/Engine/EditorBlueprintResources/StandardMacros.IsValid` (`.UserController_4_11A49D354753C45B956708A595C981A3` (break `/Game/Common/Data/LobbyData/ST_UserList` _array_element))
          (:`Is Valid`
            (`KismetSystemLibrary.PrintString` "GM: AddUserList false" true true (struct :`G` 0.66 :`B` 1.0 :`A` 1.0) 60.0))
          (:`Is Not Valid`
            (`KismetArrayLibrary.Array_Set` _userlist _array_index (make `/Game/Common/Data/LobbyData/ST_UserList` NewUserName NewUserController true))
            (`self.UpdateSessionUserList`)
            ;[1 1 1] 서버는 OnRep이 안되기에 직접 호출
            (`/Game/Common/GameMode/Lobby/BP_LobbyGameState_YJ.EventDispatcher_UserList` (`local.GameState`))
            (return)))))
    (:`CastFailed`
      (`KismetSystemLibrary.PrintString` "GM: GS cast failed"))))

(fn `UserConstructionScript`)