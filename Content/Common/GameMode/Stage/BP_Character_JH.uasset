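; Playable stage character for a cooking game that moves, carries objects and cooks at interactables.
; Grab and cook inputs sphere-trace ahead and message the hit actor through Req/Res event pairs; grabbed objects attach to Hands.
; SetIsCooking stores the interacting object and toggles an extra input mapping context for stopping.
; BeginPlay assigns materials by stage-controller index, while Tick repeatedly points player 0's view at the first CameraActor.
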(event `self.ReceiveBeginPlay`
  (bind _outactors (`GameplayStatics.GetAllActorsOfClass` "BP_Character_JH_C"))
  (for _array_element _outactors
    (`self.ReqSetMaterial` _array_element (`self.GetController` _array_element) 0)))

(event `ReqSetMaterial`
  (params (InController :type "Controller Object Reference") (Index :type Integer))
  (bind _outactors (`GameplayStatics.GetAllActorsOfClass` "/Game/Common/GameMode/Stage/BP_StageController_YJ.BP_StageController_YJ_C"))
  (for (_array_element _array_index) _outactors
    (if (== _array_element InController)
      (`self.ResSetMaterial` _array_index))))

(event `ResSetMaterial`
  (params (Index :type Integer))
  (for (_array_element _array_index) (`self.Materials`)
    (if (== _array_index Index)
      (`PrimitiveComponent.SetMaterial` (`self.Character`) 0 _array_element))))

(event `self.ReceiveTick`
  (params (DeltaSeconds :type "Float (single-precision)"))
  (bind _outactors (`GameplayStatics.GetAllActorsOfClass` "/Script/Engine.CameraActor"))
  (`PlayerController.SetViewTargetWithBlend` (`GameplayStatics.GetPlayerController` 0) (`|GetArrayItem` _outactors) 0.0 "VTBlend_Linear" 0.0 false))

(event `EnhancedInput|/Game/Common/Input/Stage/IA_Move_JH`
  (params (ActionValue :type "Vector2D Structure") (ElapsedSeconds :type "Float (double-precision)") (TriggeredSeconds :type "Float (double-precision)") (InputAction :type "InputAction Object Reference" :default "/Game/Common/Input/Stage/IA_Move_JH.IA_Move_JH"))
  ;[1 1 1] 캐릭터 기본 움직임
  (:`Triggered`
    (`self.AddMovementInput` (`KismetMathLibrary.Conv_Vector2DToVector` ActionValue))))

(event `EnhancedInput|/Game/Common/Input/Stage/IA_Grab_JH`
  (params (ActionValue :type Boolean) (ElapsedSeconds :type "Float (double-precision)") (TriggeredSeconds :type "Float (double-precision)") (InputAction :type "InputAction Object Reference" :default "/Game/Common/Input/Stage/IA_Grab_JH.IA_Grab_JH"))
  ;[1 1 1] 상호작용(스페이스바)으로 개체 그랩
  (:`Started`
    (`self.ReqGrabAndDrop`)))

(event `ReqGrabAndDrop`
  ;[1 1 1] 상호작용(스페이스바)으로 개체 그랩
  (bind (_returnvalue _outhit) (`self.GrabAndDrop` "TraceTypeQuery4"))
  (`self.ResGrabAndDrop` _returnvalue _outhit))

(event `ResGrabAndDrop`
  (params (ReturnValue :type Boolean) (OutHit :type "HitResult Structure"))
  (bind (_isgetgrabbedobject _grabbedobject) (`self.Get Grabbed Object`))
  ;[1 1 1] 상호작용(스페이스바)으로 개체 그랩
  (if ReturnValue
    (message `/Game/Common/Data/BPI_Interactable_JH.GrabAndDrop` (`.HitActor` (`GameplayStatics.BreakHitResult` OutHit)) self)
    (elif _isgetgrabbedobject
      (if (`KismetSystemLibrary.IsValid` (`self.ObjectPlace`))
        (`/Game/Common/Blueprint/Interactable/Grabbable/BP_Grabbable_JH.Drop` _grabbedobject)
        (set `self.GrabbedObject` null)))))

(event `Grab`
  (params (ObjectToGrab :type "/Game/Common/Blueprint/Interactable/Grabbable/BP_Grabbable_JH Object Reference"))
  (bind _output_get (set `self.GrabbedObject` ObjectToGrab))
  (`self.K2_AttachToComponent` _output_get (`self.Hands`) "None" "KeepWorld" "KeepWorld" "KeepWorld" true)
  (`KismetSystemLibrary.MoveComponentTo` (`Actor.RootComponent` (`self.GrabbedObject`)) (0.0 0.0 0.0) (struct :`Yaw` 270.0)))

(event `ResCooking`
  (params (ReturnValue :type Boolean) (OutHit :type "HitResult Structure"))
  (if ReturnValue
    (message `/Game/Common/Data/BPI_Interactable_JH.Cooking` (`.HitActor` (`GameplayStatics.BreakHitResult` OutHit)) self)))

(event `EnhancedInput|/Game/Common/Input/Stage/IA_Cooking_JH`
  (params (ActionValue :type Boolean) (ElapsedSeconds :type "Float (double-precision)") (TriggeredSeconds :type "Float (double-precision)") (InputAction :type "InputAction Object Reference" :default "/Game/Common/Input/Stage/IA_Cooking_JH.IA_Cooking_JH"))
  (:`Started`
    (if (not (`self.IsCooking`))
      (`self.ReqCooking`)))
  (:`Completed`
    (if (`self.IsCooking`)
      (`self.ReqStopCooking`))))

(event `ReqCooking`
  (bind (_returnvalue _outhit) (`self.GrabAndDrop` "TraceTypeQuery4"))
  (`self.ResCooking` _returnvalue _outhit))

(event `EnhancedInput|/Game/Common/Input/Stage/IA_StopInteraction_JH`
  (params (ActionValue :type Boolean) (ElapsedSeconds :type "Float (double-precision)") (TriggeredSeconds :type "Float (double-precision)") (InputAction :type "InputAction Object Reference" :default "/Game/Common/Input/Stage/IA_StopInteraction_JH.IA_StopInteraction_JH"))
  (:`Started`
    (`self.ReqStopCooking`)))

(event `ResStopCooking`
  (`self.StopCooking`))

(event `StopCooking`
  (`/Game/Common/Data/BPI_Interactable_JH.StopCooking` (`self.InteractingObject`)))

(event `ReqStopCooking`
  (`self.ResStopCooking`))

(event `SetIsCooking`
  (params (IsCooking :type Boolean) (InteractingObject :type "/Game/Common/Data/BPI_Interactable_JH Interface"))
  (bind _returnvalue (pcsubsystem `EnhancedInputLocalPlayerSubsystem` (`GameplayStatics.GetPlayerController` 0)))
  (set `self.IsCooking` IsCooking)
  (set `self.InteractingObject` InteractingObject)
  (if (`self.IsCooking`)
    (`EnhancedInputSubsystemInterface.AddMappingContext` _returnvalue "/Game/Common/Input/Stage/IMC_Interacting_JH.IMC_Interacting_JH" 0 (struct))
    (else
      (`EnhancedInputSubsystemInterface.RemoveMappingContext` _returnvalue "/Game/Common/Input/Stage/IMC_Interacting_JH.IMC_Interacting_JH" (struct)))))

(fn `Get Grabbed Object`
  (returns (IsGetGrabbedObject :type Boolean) (GrabbedObject :type "/Game/Common/Blueprint/Interactable/Grabbable/BP_Grabbable_JH Object Reference"))
  (bind _grabbedobject (`self.GrabbedObject`))
  (return (`KismetSystemLibrary.IsValid` _grabbedobject) _grabbedobject))

(fn `Get Grabbed Plate`
  (returns (ReturnValue :type Boolean) (Plate :type "/Game/Common/Blueprint/Interactable/Grabbable/BP_Plate_SH Object Reference"))
  (bind _plate (`self.Plate`))
  (return (`KismetSystemLibrary.IsValid` _plate) _plate))

(fn `GrabAndDrop`
  (params (TraceChannel :type "ETraceTypeQuery Enum" :default "TraceTypeQuery1"))
  (returns (ReturnValue :type Boolean) (OutHit :type "HitResult Structure"))
  (bind _x (.x (+ (* (`self.GetActorForwardVector`) 60.0) (`self.K2_GetActorLocation`))))
  (bind _y (.y (+ (* (`self.GetActorForwardVector`) 60.0) (`self.K2_GetActorLocation`))))
  (bind _z (.z (+ (* (`self.GetActorForwardVector`) 60.0) (`self.K2_GetActorLocation`))))
  (bind (_outhit _returnvalue) (`KismetSystemLibrary.SphereTraceSingle` (`KismetMathLibrary.MakeVector` _x _y (+ _z -80.0)) (`KismetMathLibrary.MakeVector` _x _y (+ _z 20.0)) 30.0 TraceChannel false (`|MakeArray` (`self.GrabbedObject`) :!type "Actor Object Reference") "ForDuration"))
  (return _returnvalue _outhit))

(fn `UserConstructionScript`)