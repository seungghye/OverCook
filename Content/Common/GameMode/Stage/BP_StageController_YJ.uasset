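; Player controller for stages that enables or disables input on the controlled pawn according to the stage state.
; On BeginPlay it binds to the stage game state's dispatcher, retrying by timer until the cast succeeds, then applies the current state.
; Input is enabled during Play and disabled during Ready and Score Board.
; Debug keys F and G ask the game mode to add an ordered recipe or submit a failed salad order.
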(event EventBeginPlay
  (CallFunction|BindGameState))

(event Input|KeyboardEvents|DebugKeyF
  (params (Key :type Key%20Structure) (ActionValue :type Input%20Action%20Value%20Structure))
  (:Pressed
    (bind _asbp_stage_game_mode_yj (Utilities|Casting|CastToBP_StageGameMode_YJ (Game|GetGameMode)))
    (Default|AddOrderedRecipe _asbp_stage_game_mode_yj)))

(event Input|KeyboardEvents|DebugKeyG
  (params (Key :type Key%20Structure) (ActionValue :type Input%20Action%20Value%20Structure))
  (:Pressed
    (bind _asbp_stage_game_mode_yj (Utilities|Casting|CastToBP_StageGameMode_YJ (Game|GetGameMode)))
    (Default|SubmitFood _asbp_stage_game_mode_yj "/Game/Common/Data/Recipe/DA_TomatoCabbageSalad_Recipe.DA_TomatoCabbageSalad_Recipe" false)))

(fn ConstructionScript)

(fn BindGameState
  (bind _asbp_stage_game_state_yj (Utilities|Casting|CastToBP_StageGameState_YJ (Game|GetGameState))
    (:then
      (EventDispatchers|BindEventtoEventDispatcherStageState _asbp_stage_game_state_yj (EventDispatchers|CreateEvent :!event SetControllerInput))
      (CallFunction|SetControllerInput (Variables|/Game/Common/GameMode/Stage/BP_StageGameState_YJ.BP_StageGameState_YJ_C|GetStageState _asbp_stage_game_state_yj)))
    (:CastFailed
      (Utilities|Time|SetTimerbyFunctionName 0 "BindGameState" 0.1))))

(fn SetControllerInput
  (params (StageState :type EN_StageState%20Enum :default "NewEnumerator0"))
  (bind _self self)
  (bind _self_2 self)
  (bind _self_3 self)
  (bind _returnvalue (Pawn|GetControlledPawn _self_2))
  (switch Utilities|FlowControl|Switch|SwitchonEN_StageState StageState
    (:NewEnumerator0
      (Utilities|IsValid _returnvalue
        (:Is%20Valid
          (Input|DisableInput _returnvalue _self_2))))
    (:NewEnumerator1
      (Input|EnableInput (Pawn|GetControlledPawn _self) _self))
    (:NewEnumerator2
      (Input|DisableInput (Pawn|GetControlledPawn _self_3) _self_3))))