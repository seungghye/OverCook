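; Stage GameState that holds the countdown time, score and list of ordered recipes for a stage.
; LeftTime and Score are RepNotify variables whose OnRep functions fire event dispatchers with the new values.
; Recipe orders, capped at five, are added through an event or duplicate function and removed by index, each change firing a dispatcher.
; Notes flag a possible race with HUD binding and a planned multicast conversion for removal.
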(event `ResAddOrderedRecipe`
  (params (OrderedRecipe :type "/Game/Common/Data/Recipe/DA_Recipe_BP Object Reference"))
  (bind _orderedrecipelist (`self.OrderedRecipeList`))
  (if (< (`KismetArrayLibrary.Array_Length` _orderedrecipelist) 5)
    (`KismetArrayLibrary.Array_Add` _orderedrecipelist OrderedRecipe)
    ;[1 1 1] 시작후 HUD바인드 되기 전에 호출될까봐 걱정된다. 예외처리 필요할듯
    (`self.EventDispatcher_AddOrderedRecipe` OrderedRecipe)))

(fn `AddOrderedRecipe`
  (params (OrdededRecipe :type "/Game/Common/Data/Recipe/DA_Recipe_BP Object Reference (by ref)"))
  (bind _orderedrecipelist (`self.OrderedRecipeList`))
  (if (< (`KismetArrayLibrary.Array_Length` _orderedrecipelist) 5)
    (`KismetArrayLibrary.Array_Add` _orderedrecipelist OrdededRecipe)
    ;[1 1 1] 시작후 HUD바인드 되기 전에 호출될까봐 걱정된다. 예외처리 필요할듯
    (`self.EventDispatcher_AddOrderedRecipe` OrdededRecipe)))

(fn `AddScore`
  (params (InScore :type Integer))
  (set `self.Score` (+ (`self.Score`) InScore)))

(fn `DecreaseLeftTime`
  (set `self.LeftTime` (- (`self.LeftTime`) 1)))

(fn `OnRep_LeftTime`
  (`self.EventDispatcher_LeftTime` (`self.LeftTime`)))

(fn `OnRep_Score`
  (`self.EventDispatcher_Score` (`self.Score`)))

(fn `SubtractOrderedRecipe`
  (params (RecipeIndex :type Integer))
  ;[1 1 1] Res Multicast로 HUD에 뿌리도록 이벤트로 바꾸기
  (`KismetArrayLibrary.Array_Remove` (`self.OrderedRecipeList`) RecipeIndex)
  (`self.EventDispatcher_SubtractOrderedRecipe` RecipeIndex))

(fn `UserConstructionScript`)